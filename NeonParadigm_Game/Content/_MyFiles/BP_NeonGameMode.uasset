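; BP_NeonGameMode is a game mode Blueprint with prototype FMOD music beat tracking.
; A beat handler prints bar, beat and tempo to screen as debug text.
; Setup that caches the BP_Clair_NeonParadigm player and binds the handler to BP_FMOD_Music's timeline beat event is disconnected.
; BeginPlay and Tick are empty, so nothing here performs that binding at runtime.
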(event `self.ReceiveBeginPlay`)

(event `OnTimelineBeat`
  (params (Bar :type Integer) (Beat :type Integer) (Position :type Integer) (Tempo :type "Float (single-precision)") (TimeSignatureUpper :type Integer) (TimeSignatureLower :type Integer))
  (`KismetSystemLibrary.PrintString` (`KismetStringLibrary.Conv_IntToString` Bar) true true (struct :`R` 1.0 :`B` 0.019565 :`A` 1.0) 1.0)
  (`KismetSystemLibrary.PrintString` (`KismetStringLibrary.Conv_IntToString` Beat) true true (struct :`G` 0.66 :`B` 1.0 :`A` 1.0) 1.0)
  (`KismetSystemLibrary.PrintString` (`KismetStringLibrary.Conv_DoubleToString` Tempo) true true (struct :`G` 1.0 :`B` 0.285351 :`A` 1.0) 1.0))

(fn `UserConstructionScript`)