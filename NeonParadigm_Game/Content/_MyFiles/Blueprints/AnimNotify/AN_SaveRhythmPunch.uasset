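; Anim notify that triggers the rhythm punch save on the BP_Clair_NeonParadigm character when an animation reaches it.
; It casts the mesh owner to that character, then calls its SaveRhythmPunch function.
; Debug prints flag a missing anim instance or active montage and output a "Hello" message.
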(fn `Received_Notify`
  (params (MeshComp :type "SkeletalMeshComponent Object Reference") (Animation :type "AnimSequenceBase Object Reference") (EventReference :type "AnimNotifyEventReference Structure (by ref)"))
  (returns (ReturnValue :type Boolean))
  (bind _asbp_clair_neon_paradigm (cast `/Game/_MyFiles/Blueprints/BP_Clair_NeonParadigm` (`ActorComponent.GetOwner` MeshComp)))
  (bind _returnvalue (`SkeletalMeshComponent.GetAnimInstance` (`Character.Mesh` _asbp_clair_neon_paradigm)))
  (`/Engine/EditorBlueprintResources/StandardMacros.IsValid` _returnvalue
    (:`Is Valid`
      _)
    (:`Is Not Valid`
      (`KismetSystemLibrary.PrintString` "No Anim Instance" true true (struct :`R` 1.0 :`B` 0.007701 :`A` 1.0))))
  (`/Engine/EditorBlueprintResources/StandardMacros.IsValid` (`AnimInstance.GetCurrentActiveMontage` _returnvalue)
    (:`Is Valid`
      _)
    (:`Is Not Valid`
      (`KismetSystemLibrary.PrintString` "No current Active montage" true true (struct :`R` 1.0 :`B` 0.007701 :`A` 1.0))))
  (`KismetSystemLibrary.PrintString` "Hello")
  (`/Game/_MyFiles/Blueprints/BP_Clair_NeonParadigm.SaveRhythmPunch` _asbp_clair_neon_paradigm)
  (return true))