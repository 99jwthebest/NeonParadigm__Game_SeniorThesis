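; Anim notify state that lets the player character (BP_NeonParadigm_Clair) rotate during a root motion animation for the length of the notify window.
; On begin, it enables AllowPhysicsRotationDuringAnimRootMotion on the character movement, but only when the character is not targeting and has no valid soft target actor.
; On end, it always turns the flag back off.
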(fn `Received_NotifyBegin`
  (params (MeshComp :type "SkeletalMeshComponent Object Reference") (Animation :type "AnimSequenceBase Object Reference") (TotalDuration :type "Float (single-precision)") (EventReference :type "AnimNotifyEventReference Structure (by ref)"))
  (returns (ReturnValue :type Boolean))
  (bind _asbp_neon_paradigm_clair (cast `/Game/_MyFiles/Blueprints/BP_NeonParadigm_Clair` (`ActorComponent.GetOwner` MeshComp)))
  (if (and (not (`/Game/_MyFiles/Blueprints/BP_NeonParadigm_Clair.bIsTargeting` _asbp_neon_paradigm_clair)) (not (`KismetSystemLibrary.IsValid` (`/Game/_MyFiles/Blueprints/BP_NeonParadigm_Clair.SoftTargetActor` _asbp_neon_paradigm_clair))))
    (set `CharacterMovementComponent.bAllowPhysicsRotationDuringAnimRootMotion` true (`Character.CharacterMovement` _asbp_neon_paradigm_clair))
    (return true)
    (else
      (return true))))

(fn `Received_NotifyEnd`
  (params (MeshComp :type "SkeletalMeshComponent Object Reference") (Animation :type "AnimSequenceBase Object Reference") (EventReference :type "AnimNotifyEventReference Structure (by ref)"))
  (returns (ReturnValue :type Boolean))
  (bind _asbp_neon_paradigm_clair (cast `/Game/_MyFiles/Blueprints/BP_NeonParadigm_Clair` (`ActorComponent.GetOwner` MeshComp)))
  (set `CharacterMovementComponent.bAllowPhysicsRotationDuringAnimRootMotion` false (`Character.CharacterMovement` _asbp_neon_paradigm_clair))
  (return true))