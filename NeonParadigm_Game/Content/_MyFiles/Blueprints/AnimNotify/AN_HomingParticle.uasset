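; Anim notify that fires the homing particle Niagara effect from the player's weapon socket during an animation.
; It runs only when the mesh owner is BP_Player_NeonParadigm and spawns NS_HomingParticles at WeaponSocket.
; With a valid camera target, it rotates the system toward that actor and passes its location as the Homing Target variable.
; Otherwise, the Homing Target becomes a fixed point ahead of the player along the forward vector.
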(fn `Received_Notify`
  (params (MeshComp :type "SkeletalMeshComponent Object Reference") (Animation :type "AnimSequenceBase Object Reference") (EventReference :type "AnimNotifyEventReference Structure (by ref)"))
  (returns (ReturnValue :type Boolean))
  (bind _asbp_player_neon_paradigm (cast `/Game/_MyFiles/Blueprints/BP_Player_NeonParadigm` (`ActorComponent.GetOwner` MeshComp)))
  (bind _returnvalue (`NeonParadigm_GameCharacter.GetCameraTargetActor` _asbp_player_neon_paradigm))
  (`/Engine/EditorBlueprintResources/StandardMacros.IsValid` _returnvalue
    (:`Is Valid`
      (bind _returnvalue_2 (`SceneComponent.GetSocketLocation` (`Character.Mesh` _asbp_player_neon_paradigm) "WeaponSocket"))
      (bind _returnvalue_3 (`Actor.K2_GetActorLocation` _asbp_player_neon_paradigm))
      (bind _returnvalue_4 (`Actor.K2_GetActorLocation` _returnvalue))
      (bind _returnvalue_5 (`NiagaraFunctionLibrary.SpawnSystemAtLocation` "/Game/_MyFiles/RyanVFX/NS/NS_HomingParticles.NS_HomingParticles" _returnvalue_2 (`KismetMathLibrary.FindLookAtRotation` _returnvalue_3 _returnvalue_4)))
      (`NiagaraComponent.SetVariableVec3` _returnvalue_5 "Homing Target" _returnvalue_4)
      (return true))
    (:`Is Not Valid`
      (bind _returnvalue_6 (`NiagaraFunctionLibrary.SpawnSystemAtLocation` "/Game/_MyFiles/RyanVFX/NS/NS_HomingParticles.NS_HomingParticles" _returnvalue_2))
      (`NiagaraComponent.SetVariableVec3` _returnvalue_6 "Homing Target" (+ _returnvalue_3 (* (`Actor.GetActorForwardVector` _asbp_player_neon_paradigm) 650.0))))))