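; Ranged enemy test Blueprint that attacks the player with magic shots or an energy beam and plays a falling death for flying AI.
; FireProjectile spawns BP_MagicShot toward the player, registering itself as the player's projectile-counter location.
; RotateToTarget caches player position, so DrawLaserProjectile's sphere-traced beam damages along a lagged, dodgeable aim.
; Damage triggers delayed AttackMovement; a looping timer shrinks the capsule and lowers the mesh on death.
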(event `self.ReceiveBeginPlay`
  (`parent.ReceiveBeginPlay`))

(event `self.ReceiveAnyDamage`
  (params (Damage :type "Float (single-precision)") (DamageType :type "DamageType Object Reference") (InstigatedBy :type "Controller Object Reference") (DamageCauser :type "Actor Object Reference"))
  ;[1 0 0] THIS IS TERRIBLE LMAO. FIX THIS WHEN GET A CHANCERS
  (`KismetSystemLibrary.Delay` 0.15)
  (`self.AttackMovement` -10.0))

(event `self.ReceiveTick`
  (params (DeltaSeconds :type "Float (single-precision)"))
  (`parent.ReceiveTick` DeltaSeconds))

(event `FireProjectile`
  (bind (_returnvalue_location _returnvalue_rotation _returnvalue_scale) (`KismetMathLibrary.BreakTransform` (`self.GetTransform`)))
  (bind _returnvalue (`GameplayStatics.GetPlayerCharacter` 0))
  (`|SpawnActorFromClass` "/Game/_MyFiles/Blueprints/Projectiles/BP_MagicShot.BP_MagicShot_C" (`KismetMathLibrary.MakeTransform` _returnvalue_location (`KismetMathLibrary.FindLookAtRotation` (`self.K2_GetActorLocation`) (`self.K2_GetActorLocation` _returnvalue)) _returnvalue_scale) "AdjustIfPossibleButAlwaysSpawn" "MultiplyWithRoot" self null)
  (bind _asbp_player_neon_paradigm (cast `/Game/_MyFiles/Blueprints/BP_Player_NeonParadigm` _returnvalue))
  (set `/Game/_MyFiles/Blueprints/BP_Player_NeonParadigm.ProjectileCounterActorLoc` self _asbp_player_neon_paradigm))

(event `StartFlyingAiDeath`
  (bind _returnvalue (`KismetSystemLibrary.K2_SetTimerDelegate` (delegate `FlyingAIDeath`) (`GameplayStatics.GetWorldDeltaSeconds`) true))
  (set `self.FlyingDeathAiTimer` _returnvalue)
  (`AnimInstance.SetRootMotionMode` (`SkeletalMeshComponent.GetAnimInstance` (`self.Mesh`)) "IgnoreRootMotion"))

(event `FlyingAIDeath`
  (bind _returnvalue (`GameplayStatics.GetWorldDeltaSeconds`))
  (bind _capsulecomponent (`self.CapsuleComponent`))
  (bind _staticmesh (`self.StaticMesh`))
  (bind _returnvalue_2 (`KismetMathLibrary.FInterpTo_Constant` (`CapsuleComponent.CapsuleHalfHeight` _capsulecomponent) 34.0 _returnvalue (`self.FallingDeathSpeed`)))
  (bind (_returnvalue_x _returnvalue_y _returnvalue_z) (`KismetMathLibrary.BreakVector` (`KismetMathLibrary.VInterpTo_Constant` (`SceneComponent.RelativeLocation` _staticmesh) (0.0 0.0 -165.0) _returnvalue (`self.FallingDeathSpeed`))))
  (`CapsuleComponent.SetCapsuleHalfHeight` _capsulecomponent _returnvalue_2 true)
  (if (< _returnvalue_2 34.5)
    (`SceneComponent.K2_SetRelativeLocation` _staticmesh (`KismetMathLibrary.MakeVector` _returnvalue_x _returnvalue_y _returnvalue_z) false false)
    (if (<= _returnvalue_z -160.0)
      (`KismetSystemLibrary.K2_ClearAndInvalidateTimerHandle` (`self.FlyingDeathAiTimer`)))))

(fn `DrawLaserProjectile`
  (params (Radius :type "Float (double-precision)") (DamageTypeClass :type "NP_DamageType Class Reference") (AmountOfDamage :type "Float (double-precision)"))
  (locals (Direction :type "Vector Structure") (BeamRotation :type "Rotator Structure"))
  (bind _playerdelayedlocation (`self.PlayerDelayedLocation`))
  (bind _returnvalue (`SceneComponent.K2_GetComponentLocation` (`self.WeaponMesh`)))
  (`KismetArrayLibrary.Array_Clear` (`self.HitActors`))
  (bind _output_get (set `local.Direction` (`KismetMathLibrary.Normal` (- _returnvalue _playerdelayedlocation))))
  (bind _output_get_2 (set `local.BeamRotation` (`KismetMathLibrary.Conv_VectorToRotator` _output_get)))
  (`NiagaraFunctionLibrary.SpawnSystemAtLocation` "/Game/_MyFiles/RyanVFX/NS/NS_EnergyBeam.NS_EnergyBeam" _returnvalue (`KismetMathLibrary.MakeRotator` (.roll _output_get_2) (+ (.pitch _output_get_2) 90.0) (.yaw _output_get_2)))
  ;[0.02083 0.02083 0.02083] Collision
  (bind (_outhits _returnvalue_2) (`KismetSystemLibrary.SphereTraceMultiForObjects` :`Start` _returnvalue :`End` _playerdelayedlocation :`Radius` Radius :`ObjectTypes` (`|MakeArray` "ObjectTypeQuery3" :!type "EObjectTypeQuery Enum") :`DrawDebugType` "ForDuration"))
  (if _returnvalue_2
    ;[0.02083 0.02083 0.02083] Check Each Actor Hit
    (for _array_element _outhits
      (bind (_bblockinghit _binitialoverlap _time _distance _location _impactpoint _normal _impactnormal _physmat _hitactor) (`GameplayStatics.BreakHitResult` _array_element))
      ;[0.02083 0.02083 0.02083] Hit Actor Cannot Be In The Array and Has To Be Valid To Take Damage
      (if (and (not (`KismetArrayLibrary.Array_Contains` (`self.HitActors`) _hitactor)) (`KismetSystemLibrary.IsValid` _hitactor))
        (bind _asbp_player_neon_paradigm (cast `/Game/_MyFiles/Blueprints/BP_Player_NeonParadigm` _hitactor))
        (if (`|EnumInequality` (`CharacterStateComponent.GetState` (`NeonParadigm_GameCharacter.CharacterState` _asbp_player_neon_paradigm)) "Death")
          (`GameplayStatics.ApplyDamage` _hitactor (`local.AmountOfDamage`) (`self.GetController`) self (`local.DamageTypeClass`))
          (`KismetArrayLibrary.Array_AddUnique` (`self.HitActors`) _hitactor))))))

(fn `RotateToTarget`
  (params (InDeltaTime :type "Float (double-precision)") (InRotationSpeed :type "Float (double-precision)"))
  (bind _returnvalue (`self.K2_GetActorLocation`))
  (bind _returnvalue_2 (`self.K2_GetActorLocation` (`GameplayStatics.GetPlayerCharacter` 0)))
  (`self.K2_SetActorRotation` (`KismetMathLibrary.RInterpTo` (`self.K2_GetActorRotation`) (`KismetMathLibrary.FindLookAtRotation` (`self.K2_GetActorLocation`) _returnvalue_2) InDeltaTime InRotationSpeed))
  (set `self.PlayerDelayedLocation` _returnvalue_2)
  (`KismetSystemLibrary.SphereTraceMultiForObjects` :`Start` _returnvalue :`End` (+ _returnvalue (* (`self.GetActorForwardVector`) 800.0)) :`Radius` 80.0 :`ObjectTypes` (`|MakeArray` "ObjectTypeQuery3" :!type "EObjectTypeQuery Enum") :`DrawDebugType` "ForDuration" :`DrawTime` 1.0))

(fn `UserConstructionScript`
  (`parent.UserConstructionScript`))