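; Euphony boss character with a health bar on the player HUD, difficulty-scaled damage intake and death handling.
; Construction attaches arm, body and tentacle hitboxes to skeleton sockets and maps each to a damage multiplier, which attacks can temporarily lower.
; Attack functions (slams, tentacles, projectiles, rotate stun) mostly sphere-trace, then damage, knock back and briefly disable player root motion.
; Helpers handle emissive attack cues, turning and hand collision.
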(event `self.ReceiveBeginPlay`
  (`KismetSystemLibrary.Delay` 0.02)
  (bind _returnvalue (`|CreateWidget` "/Game/_MyFiles/UI/WBP_BossHealthBar.WBP_BossHealthBar_C"))
  (bind _output_get (set `self.BossHealthBarWidget` _returnvalue))
  (set `/Game/_MyFiles/UI/WBP_BossHealthBar.EnemyBossOwner` self _output_get)
  (`/Game/_MyFiles/UI/WBP_BossHealthBar.UpdateHealth` _output_get)
  (bind _asbp_player_neon_paradigm (cast `/Game/_MyFiles/Blueprints/BP_Player_NeonParadigm` (`GameplayStatics.GetPlayerCharacter` 0)))
  (`VerticalBox.AddChildToVerticalBox` (`/Game/_MyFiles/UI/WBP_HUD.BossVerticalBox` (`/Game/_MyFiles/Blueprints/BP_Player_NeonParadigm.HudWidget` _asbp_player_neon_paradigm)) (`self.BossHealthBarWidget`))
  (`self.InitializeEmissiveMatInstances`)
  (bind _asabp_boss_euphony_new (cast `/Game/_MyFiles/Animation/Blueprints/ABP_Boss_Euphony_New` (`SkeletalMeshComponent.GetAnimInstance` (`self.Mesh`))))
  (set `self.As ABP Boss Euphony New` _asabp_boss_euphony_new)
  (bind _asbp_np_game_instance (cast `/Game/_MyFiles/Blueprints/GameInstance/BP_NP_GameInstance` (`GameplayStatics.GetGameInstance`)))
  (set `self.As BP NP Game Instance` _asbp_np_game_instance)
  (switch `int` (`NP_GameInstance.GetCurrentDifficultyMode` (`self.As BP NP Game Instance`))
    (:`0`
      (set `self.BaseDamageMultiplier` 1.0))
    (:`1`
      (set `self.BaseDamageMultiplier` 0.5))
    (:`2`
      (set `self.BaseDamageMultiplier` 0.25))))

(event `self.ReceiveAnyDamage`
  (params (Damage :type "Float (single-precision)") (DamageType :type "DamageType Object Reference") (InstigatedBy :type "Controller Object Reference") (DamageCauser :type "Actor Object Reference"))
  (bind _hitboxdamagemultipliers (`self.HitBoxDamageMultipliers`))
  (if (> (`self.CurrentHealth`) 0.0)
    (if (`KismetSystemLibrary.IsValid` DamageCauser)
      (bind _asbp_player_neon_paradigm (cast `/Game/_MyFiles/Blueprints/BP_Player_NeonParadigm` DamageCauser))
      (`/Engine/EditorBlueprintResources/StandardMacros.IsValid` _asbp_player_neon_paradigm
        (:`Is Valid`
          (bind _output_get (set `self.PlayersLastHitBox` (`DamageComponent.LastHitResult` (`NeonParadigm_GameCharacter.DamageComp` _asbp_player_neon_paradigm))))
          (`/Engine/EditorBlueprintResources/StandardMacros.IsValid` (`.HitComponent` (`GameplayStatics.BreakHitResult` _output_get))
            (:`Is Valid`
              (bind _output_get_2 (set `self.HitComponent` (`.HitComponent` (`GameplayStatics.BreakHitResult` _output_get))))
              (if (`BlueprintMapLibrary.Map_Contains` _hitboxdamagemultipliers _output_get_2)
                (bind _output_get_3 (set `self.DamageMultiplier` (`BlueprintMapLibrary.Map_Find` _hitboxdamagemultipliers _output_get_2)))
                (bind _output_get_4 (set `self.FinalDamage` (* (* _output_get_3 (`self.BaseDamageMultiplier`)) Damage)))
                (set `self.CurrentHealth` (- (`self.CurrentHealth`) _output_get_4))
                (`KismetSystemLibrary.Delay` 0.02)
                (`/Game/_MyFiles/UI/WBP_BossHealthBar.UpdateHealth` (`self.BossHealthBarWidget`))
                (`NiagaraFunctionLibrary.SpawnSystemAtLocation` "/Game/_MyFiles/VFX/NS_EuphonyEnergyBlood.NS_EuphonyEnergyBlood" (`SceneComponent.K2_GetComponentLocation` (`self.HitComponent`)) (struct) (3.0 3.0 3.0))))))))
    (else
      (`self.PerformDeath`)
      (bind _asbp_player_neon_paradigm_2 (cast `/Game/_MyFiles/Blueprints/BP_Player_NeonParadigm` (`GameplayStatics.GetPlayerCharacter` 0)))
      (set `/Game/_MyFiles/Blueprints/BP_Player_NeonParadigm.BP_Euphony` self _asbp_player_neon_paradigm_2))))

(fn `AttachCollidersToTentacles`
  (params (Target1 :type "SceneComponent Object Reference") (SocketName1 :type Name) (Target2 :type "SceneComponent Object Reference") (SocketName2 :type Name) (Target3 :type "SceneComponent Object Reference") (SocketName3 :type Name) (Target4 :type "SceneComponent Object Reference") (SocketName4 :type Name))
  (bind _mesh (`self.Mesh`))
  (`SceneComponent.K2_AttachToComponent` Target1 _mesh SocketName1 "KeepRelative" "KeepRelative" "KeepRelative" true)
  (`SceneComponent.K2_AttachToComponent` Target2 _mesh SocketName2 "KeepRelative" "KeepRelative" "KeepRelative" true)
  (`SceneComponent.K2_AttachToComponent` Target3 _mesh SocketName3 "KeepRelative" "KeepRelative" "KeepRelative" true)
  (`SceneComponent.K2_AttachToComponent` Target4 _mesh SocketName4 "KeepRelative" "KeepRelative" "KeepRelative" true))

(fn `ChangeDamageMultipliers`
  (params (`ReturnToDefaultValues?` :type Boolean) (BossAttackTypeEnum :type "/Game/_MyFiles/Blueprints/Enemies/BossAttackTypes Enum" :default "NewEnumerator0"))
  (bind _hitboxdamagemultipliers (`self.HitBoxDamageMultipliers`))
  (bind _mainbodyhitbox (`self.MainBodyHitBox`))
  (bind _finaldamgemultiplier_arms (`self.FinalDamgeMultiplier_Arms`))
  (bind _armhitbox_l (`self.ArmHitBox_L`))
  (bind _armhitbox_r (`self.ArmHitBox_R`))
  (if `ReturnToDefaultValues?`
    (switch `/Game/_MyFiles/Blueprints/Enemies/BossAttackTypes` (`local.BossAttackTypeEnum`)
      (:`NewEnumerator0`
        (`BlueprintMapLibrary.Map_Add` _hitboxdamagemultipliers _armhitbox_l _finaldamgemultiplier_arms)
        (`BlueprintMapLibrary.Map_Add` _hitboxdamagemultipliers _armhitbox_r _finaldamgemultiplier_arms))
      (:`NewEnumerator1`
        (`BlueprintMapLibrary.Map_Add` _hitboxdamagemultipliers _mainbodyhitbox (`self.FinalDamgeMultiplier_Body`))))
    (else
      (switch `/Game/_MyFiles/Blueprints/Enemies/BossAttackTypes` (`local.BossAttackTypeEnum`)
        (:`NewEnumerator0`
          (`BlueprintMapLibrary.Map_Add` _hitboxdamagemultipliers _armhitbox_l 0.01)
          (`BlueprintMapLibrary.Map_Add` _hitboxdamagemultipliers _armhitbox_r 0.01))
        (:`NewEnumerator1`
          (`BlueprintMapLibrary.Map_Add` _hitboxdamagemultipliers _mainbodyhitbox 0.05))))))

(fn `ChangeEmissiveStatePattern`
  (params (BossAttackTypes_Enum :type "/Game/_MyFiles/Blueprints/Enemies/BossAttackTypes Enum" :default "NewEnumerator0") (`StartAttack?` :type Boolean))
  (set `self.EmissiveStateValue` (select `bool` (`local.StartAttack?`) :`false` 1.0 :!type "Float (single-precision)"))
  (switch `/Game/_MyFiles/Blueprints/Enemies/BossAttackTypes` (`local.BossAttackTypes_Enum`)
    (:`NewEnumerator0`
      (`MaterialInstanceDynamic.SetScalarParameterValue` (`self.EmissiveDynMat_Arms`) "ChangingEmissivePatterns" (`self.EmissiveStateValue`)))
    (:`NewEnumerator1`
      (`MaterialInstanceDynamic.SetScalarParameterValue` (`self.EmissiveDynMat_Body`) "ChangingEmissivePatterns" (`self.EmissiveStateValue`)))
    (:`NewEnumerator2`
      (`MaterialInstanceDynamic.SetScalarParameterValue` (`self.EmissiveDynMat_Tents`) "ChangingEmissivePatterns" (`self.EmissiveStateValue`) :!label _label))
    (:`NewEnumerator3`
      (goto _label))))

(fn `InitializeEmissiveMatInstances`
  (bind _mesh (`self.Mesh`))
  (bind _mesh_2 (`self.Mesh`))
  (bind _mesh_3 (`self.Mesh`))
  (bind _returnvalue (`PrimitiveComponent.CreateDynamicMaterialInstance` _mesh_2 3 (`PrimitiveComponent.GetMaterial` _mesh_2 3) "None"))
  (set `self.EmissiveDynMat_Arms` _returnvalue)
  (bind _returnvalue_2 (`PrimitiveComponent.CreateDynamicMaterialInstance` _mesh_3 4 (`PrimitiveComponent.GetMaterial` _mesh_3 4) "None"))
  (set `self.EmissiveDynMat_Tents` _returnvalue_2)
  (bind _returnvalue_3 (`PrimitiveComponent.CreateDynamicMaterialInstance` _mesh 5 (`PrimitiveComponent.GetMaterial` _mesh 5) "None"))
  (set `self.EmissiveDynMat_Body` _returnvalue_3))

(fn `PerformBasicAttack_L`
  (locals (KnockbackDirection :type "Vector Structure") (KnockbackImpulse :type "Vector Structure") (RadiusForAttack :type "Float (double-precision)" :default 700.0))
  (bind _returnvalue (`self.K2_GetActorLocation`))
  (bind _returnvalue_2 (`SceneComponent.GetSocketLocation` (`self.Mesh`) "Wrist_L"))
  (`GameplayStatics.SpawnSoundAtLocation` "/Game/_MyFiles/Sound_FX/AI_Gen_Sounds/Euphony/Euphony_SlammingFists_2.Euphony_SlammingFists_2" _returnvalue (struct) 1.0 1.0 0.05 null null)
  (`GameplayStatics.SpawnSoundAtLocation` "/Game/_MyFiles/Sound_FX/AI_Gen_Sounds/Euphony/Euphony_SlammingFists_4.Euphony_SlammingFists_4" _returnvalue (struct) 1.0 1.0 0.05 null null)
  (bind (_outhit _returnvalue_3) (`KismetSystemLibrary.SphereTraceSingleForObjects` _returnvalue_2 _returnvalue_2 (`local.RadiusForAttack`) (`|MakeArray` "ObjectTypeQuery3" :!type "EObjectTypeQuery Enum")))
  (if _returnvalue_3
    (bind _asbp_player_neon_paradigm (cast `/Game/_MyFiles/Blueprints/BP_Player_NeonParadigm` (`GameplayStatics.GetPlayerCharacter` 0)))
    (bind _output_get (set `local.KnockbackDirection` (`KismetMathLibrary.Normal` (- (`self.K2_GetActorLocation` _asbp_player_neon_paradigm) (`self.K2_GetActorLocation`)))))
    (bind _output_get_2 (set `local.KnockbackImpulse` (* (`KismetMathLibrary.MakeVector` (.x _output_get) (.y _output_get) 0.7) (`self.BasicAttackKnockbackForce`))))
    (`KismetSystemLibrary.PrintString` (`KismetStringLibrary.Conv_VectorToString` _output_get_2))
    (`CharacterMovementComponent.AddImpulse` (`Character.CharacterMovement` _asbp_player_neon_paradigm) _output_get_2 true)
    (`AnimInstance.SetRootMotionMode` (`SkeletalMeshComponent.GetAnimInstance` (`Character.Mesh` _asbp_player_neon_paradigm)) "IgnoreRootMotion")
    (`GameplayStatics.ApplyRadialDamage` :`BaseDamage` 100.0 :`Origin` _returnvalue_2 :`DamageRadius` (`local.RadiusForAttack`) :`DamageTypeClass` "/Game/_MyFiles/Blueprints/NP_DamageTypes/NP_DT_Middle.NP_DT_Middle_C" :`DamageCauser` self :`InstigatedByController` (`self.GetInstigatorController`) :`bDoFullDamage` true)
    (bind _returnvalue_4 (`KismetSystemLibrary.K2_SetTimer` null "ReenablePlayerInput" 1.0))
    (set `self.TimerForBasicAttackReenable_L` _returnvalue_4)))

(fn `PerformBasicAttack_R`
  (locals (KnockbackDirection :type "Vector Structure") (KnockbackImpulse :type "Vector Structure") (RadiusForAttack :type "Float (double-precision)" :default 700.0))
  (bind _returnvalue (`self.K2_GetActorLocation`))
  (bind _returnvalue_2 (`SceneComponent.GetSocketLocation` (`self.Mesh`) "Wrist_R"))
  (`GameplayStatics.SpawnSoundAtLocation` "/Game/_MyFiles/Sound_FX/AI_Gen_Sounds/Euphony/Euphony_SlammingFists_2.Euphony_SlammingFists_2" _returnvalue (struct) 1.0 1.0 0.05 null null)
  (`GameplayStatics.SpawnSoundAtLocation` "/Game/_MyFiles/Sound_FX/AI_Gen_Sounds/Euphony/Euphony_SlammingFists_4.Euphony_SlammingFists_4" _returnvalue (struct) 1.0 1.0 0.05 null null)
  (bind (_outhit _returnvalue_3) (`KismetSystemLibrary.SphereTraceSingleForObjects` _returnvalue_2 _returnvalue_2 (`local.RadiusForAttack`) (`|MakeArray` "ObjectTypeQuery3" :!type "EObjectTypeQuery Enum")))
  (if _returnvalue_3
    (bind _asbp_player_neon_paradigm (cast `/Game/_MyFiles/Blueprints/BP_Player_NeonParadigm` (`GameplayStatics.GetPlayerCharacter` 0)))
    (bind _output_get (set `local.KnockbackDirection` (`KismetMathLibrary.Normal` (- (`self.K2_GetActorLocation` _asbp_player_neon_paradigm) (`self.K2_GetActorLocation`)))))
    (bind _output_get_2 (set `local.KnockbackImpulse` (* (`KismetMathLibrary.MakeVector` (.x _output_get) (.y _output_get) 0.7) (`self.BasicAttackKnockbackForce`))))
    (`KismetSystemLibrary.PrintString` (`KismetStringLibrary.Conv_VectorToString` _output_get_2))
    (`CharacterMovementComponent.AddImpulse` (`Character.CharacterMovement` _asbp_player_neon_paradigm) _output_get_2 true)
    (`AnimInstance.SetRootMotionMode` (`SkeletalMeshComponent.GetAnimInstance` (`Character.Mesh` _asbp_player_neon_paradigm)) "IgnoreRootMotion")
    (`GameplayStatics.ApplyRadialDamage` :`BaseDamage` 100.0 :`Origin` _returnvalue_2 :`DamageRadius` (`local.RadiusForAttack`) :`DamageTypeClass` "/Game/_MyFiles/Blueprints/NP_DamageTypes/NP_DT_Middle.NP_DT_Middle_C" :`DamageCauser` self :`InstigatedByController` (`self.GetInstigatorController`) :`bDoFullDamage` true)
    (bind _returnvalue_4 (`KismetSystemLibrary.K2_SetTimer` null "ReenablePlayerInput" 1.0))
    (set `self.TimerForBasicAttackReenable_R` _returnvalue_4)))

(fn `PerformEuphonyDeath`
  (`GameplayStatics.SpawnSoundAtLocation` "/Game/_MyFiles/Sound_FX/AI_Gen_Sounds/Euphony/Euphony_ShuttingDown_3.Euphony_ShuttingDown_3" (`self.K2_GetActorLocation`) (struct) 1.0 1.0 0.0 null null)
  (`GameplayStatics.SpawnSoundAtLocation` "/Game/_MyFiles/Sound_FX/AI_Gen_Sounds/Euphony/Euphony_ShuttingDown_2.Euphony_ShuttingDown_2" (`self.K2_GetActorLocation`) (struct) 1.0 1.0 0.0 null null)
  (`self.PlayAnimMontage` "/Game/_MyFiles/Animation/Assets/Euphony/Anims/AM_Euphony_Death.AM_Euphony_Death")
  (`/Game/_MyFiles/Animation/Blueprints/ABP_Boss_Euphony_New.SetAllAnimBlendWeightsToZero` (`self.As ABP Boss Euphony New`)))

(fn `PerformGroundSlamAttack`
  (locals (KnockbackDirection :type "Vector Structure") (KnockbackImpulse :type "Vector Structure"))
  (bind _returnvalue (`self.K2_GetActorLocation`))
  (bind (_outhit _returnvalue_2) (`KismetSystemLibrary.SphereTraceSingleForObjects` _returnvalue _returnvalue 2000.0 (`|MakeArray` "ObjectTypeQuery3" :!type "EObjectTypeQuery Enum")))
  (if _returnvalue_2
    (bind _asbp_player_neon_paradigm (cast `/Game/_MyFiles/Blueprints/BP_Player_NeonParadigm` (`GameplayStatics.GetPlayerCharacter` 0)))
    (bind _output_get (set `local.KnockbackDirection` (`KismetMathLibrary.Normal` (- (`self.K2_GetActorLocation` _asbp_player_neon_paradigm) (`self.K2_GetActorLocation`)))))
    (bind _output_get_2 (set `local.KnockbackImpulse` (* (`KismetMathLibrary.MakeVector` (.x _output_get) (.y _output_get) 0.7) (`self.GroundSlamKnockbackForce`))))
    (`KismetSystemLibrary.PrintString` (`KismetStringLibrary.Conv_VectorToString` _output_get_2))
    (`CharacterMovementComponent.AddImpulse` (`Character.CharacterMovement` _asbp_player_neon_paradigm) _output_get_2 true)
    (`AnimInstance.SetRootMotionMode` (`SkeletalMeshComponent.GetAnimInstance` (`Character.Mesh` _asbp_player_neon_paradigm)) "IgnoreRootMotion")
    (`GameplayStatics.ApplyRadialDamage` :`BaseDamage` (`self.GroundSlamAttackDamage`) :`Origin` _returnvalue :`DamageRadius` 2000.0 :`DamageTypeClass` "/Game/_MyFiles/Blueprints/NP_DamageTypes/NP_DT_Middle.NP_DT_Middle_C" :`DamageCauser` self :`InstigatedByController` (`self.GetInstigatorController`) :`bDoFullDamage` true)
    (bind _returnvalue_3 (`KismetSystemLibrary.K2_SetTimer` null "ReenablePlayerInput" 1.5))
    (set `self.TimerForGroundSlamReenable` _returnvalue_3)
    (`/Game/_MyFiles/Blueprints/BP_Player_NeonParadigm.PlayCameraShake` _asbp_player_neon_paradigm)))

(fn `PerformRotateStunPlayer`
  (params (`LeftHand?` :type Boolean))
  (locals (KnockbackDirection :type "Vector Structure") (KnockbackImpulse :type "Vector Structure") (RadiusForAttack :type "Float (double-precision)" :default 700.0))
  (bind _returnvalue (`SceneComponent.GetSocketLocation` (`self.Mesh`) (select `bool` `LeftHand?` :`false` "Wrist_R" :`true` "Wrist_L" :!type "Name")))
  (bind (_outhit _returnvalue_2) (`KismetSystemLibrary.SphereTraceSingleForObjects` _returnvalue _returnvalue (`local.RadiusForAttack`) (`|MakeArray` "ObjectTypeQuery3" :!type "EObjectTypeQuery Enum")))
  (if _returnvalue_2
    (bind _asbp_player_neon_paradigm (cast `/Game/_MyFiles/Blueprints/BP_Player_NeonParadigm` (`GameplayStatics.GetPlayerCharacter` 0)))
    (`AnimInstance.SetRootMotionMode` (`SkeletalMeshComponent.GetAnimInstance` (`Character.Mesh` _asbp_player_neon_paradigm)) "IgnoreRootMotion")
    (`GameplayStatics.ApplyRadialDamage` :`BaseDamage` (`self.RotateStunDamage`) :`Origin` _returnvalue :`DamageRadius` (`local.RadiusForAttack`) :`DamageTypeClass` "/Game/_MyFiles/Blueprints/NP_DamageTypes/NP_DT_Middle.NP_DT_Middle_C" :`DamageCauser` self :`InstigatedByController` (`self.GetInstigatorController`) :`bDoFullDamage` true)
    (bind _returnvalue_3 (`KismetSystemLibrary.K2_SetTimer` null "ReenablePlayerInput" 1.0))
    (set `self.TimerForBasicAttackReenable_L` _returnvalue_3)
    (`/Game/_MyFiles/Blueprints/BP_Player_NeonParadigm.PlayBossRotateStepCamerShake` _asbp_player_neon_paradigm)))

(fn `PerformShootProjectiles`
  (locals (RandomOffset :type "Vector Structure") (RandomTargetLocation :type "Vector Structure") (SpawnLocation :type "Vector Structure") (SpawnRotation :type "Rotator Structure"))
  (for _array_element (`|MakeArray` (`self.Arrow1`) (`self.Arrow2`) (`self.Arrow3`) (`self.Arrow4`) (`self.Arrow5`) (`self.Arrow6`))
    (if (not (not (`KismetSystemLibrary.IsValid` _array_element)))
      (set `local.RandomOffset` (* (`KismetMathLibrary.RandomUnitVector`) (`KismetMathLibrary.RandomFloatInRange` 0.0 (`self.TargetRadiusProjectiles`))))
      (bind _output_get (set `local.RandomTargetLocation` (+ (`self.K2_GetActorLocation` (`GameplayStatics.GetPlayerCharacter` 0)) (`local.RandomOffset`))))
      (bind _output_get_2 (set `local.SpawnLocation` (`SceneComponent.K2_GetComponentLocation` _array_element)))
      (bind _output_get_3 (set `local.SpawnRotation` (`KismetMathLibrary.FindLookAtRotation` _output_get_2 _output_get)))
      (`|SpawnActorFromClass` "/Game/_MyFiles/Blueprints/Projectiles/BP_Projectile.BP_Projectile_C" (`KismetMathLibrary.MakeTransform` _output_get_2 _output_get_3) "AdjustIfPossibleButAlwaysSpawn" "MultiplyWithRoot" self null)))
  (`KismetSystemLibrary.PrintString` "Yeah ...!!!!!"))

(fn `PerformTentacleSingleAttack`
  (params (TentacleBoneName :type Name))
  (locals (KnockbackDirection :type "Vector Structure") (KnockbackImpulse :type "Vector Structure") (RadiusForAttack :type "Float (double-precision)" :default 200.0) (ArrayOfTentacleNames :type "Array of Name"))
  (bind _mesh (`self.Mesh`))
  (bind _returnvalue (`SceneComponent.GetSocketLocation` _mesh TentacleBoneName))
  (bind (_returnvalue_location _returnvalue_rotation) (`KismetMathLibrary.BreakTransform` (`SceneComponent.GetSocketTransform` _mesh TentacleBoneName "RTS_World")))
  (bind (_outhit _returnvalue_2) (`KismetSystemLibrary.SphereTraceSingleForObjects` _returnvalue (+ _returnvalue (* (* (`KismetMathLibrary.GetForwardVector` _returnvalue_rotation) (`KismetMathLibrary.SelectFloat` 1.0 -1.0 (`KismetArrayLibrary.Array_Contains` (`local.ArrayOfTentacleNames`) TentacleBoneName))) (`self.TentacleAttack_Length`))) (`local.RadiusForAttack`) (`|MakeArray` "ObjectTypeQuery3" :!type "EObjectTypeQuery Enum")))
  (if _returnvalue_2
    (bind _asbp_player_neon_paradigm (cast `/Game/_MyFiles/Blueprints/BP_Player_NeonParadigm` (`GameplayStatics.GetPlayerCharacter` 0)))
    (bind _output_get (set `local.KnockbackDirection` (`KismetMathLibrary.Normal` (- (`self.K2_GetActorLocation` _asbp_player_neon_paradigm) (`self.K2_GetActorLocation`)))))
    (bind _output_get_2 (set `local.KnockbackImpulse` (* (`KismetMathLibrary.MakeVector` (.x _output_get) (.y _output_get) 0.7) (`self.BasicAttackKnockbackForce`))))
    (`KismetSystemLibrary.PrintString` (`KismetStringLibrary.Conv_VectorToString` _output_get_2))
    (`CharacterMovementComponent.AddImpulse` (`Character.CharacterMovement` _asbp_player_neon_paradigm) _output_get_2 true)
    (`AnimInstance.SetRootMotionMode` (`SkeletalMeshComponent.GetAnimInstance` (`Character.Mesh` _asbp_player_neon_paradigm)) "IgnoreRootMotion")
    (`GameplayStatics.ApplyRadialDamage` :`BaseDamage` 100.0 :`Origin` _returnvalue :`DamageRadius` (`local.RadiusForAttack`) :`DamageTypeClass` "/Game/_MyFiles/Blueprints/NP_DamageTypes/NP_DT_Middle.NP_DT_Middle_C" :`DamageCauser` self :`InstigatedByController` (`self.GetInstigatorController`) :`bDoFullDamage` true)
    (bind _returnvalue_3 (`KismetSystemLibrary.K2_SetTimer` null "ReenablePlayerInput" 1.0))
    (set `self.TimerForBasicAttackReenable_L` _returnvalue_3)))

(fn `ReenablePlayerInput`
  (bind _asbp_player_neon_paradigm (cast `/Game/_MyFiles/Blueprints/BP_Player_NeonParadigm` (`GameplayStatics.GetPlayerCharacter` 0)))
  (`AnimInstance.SetRootMotionMode` (`SkeletalMeshComponent.GetAnimInstance` (`Character.Mesh` _asbp_player_neon_paradigm)) "RootMotionFromEverything")
  (`KismetSystemLibrary.PrintString` "Succeedded!!!!" true true (struct :`G` 0.66 :`B` 1.0 :`A` 1.0) 20.0)
  (`KismetSystemLibrary.K2_ClearAndInvalidateTimerHandle` (`self.TimerForGroundSlamReenable`))
  (`KismetSystemLibrary.K2_ClearAndInvalidateTimerHandle` (`self.TimerForBasicAttackReenable_L`))
  (`KismetSystemLibrary.K2_ClearAndInvalidateTimerHandle` (`self.TimerForBasicAttackReenable_R`)))

(fn `RotateEuphony`
  (params (`TurnRight?` :type Boolean) (RotationSpeed :type "Float (double-precision)"))
  (locals (TargetYawRot :type "Float (single-precision)" :default 0.0) (DeltaRotation :type "Float (double-precision)") (AppliedRotation :type "Float (double-precision)"))
  (bind _rotationremaining (`self.RotationRemaining`))
  (set `self.IsRotating?` true)
  (bind _output_get (set `local.DeltaRotation` (* RotationSpeed (`GameplayStatics.GetWorldDeltaSeconds`))))
  (if (> _output_get _rotationremaining)
    (bind _output_get_2 (set `local.DeltaRotation` _rotationremaining)))
  (bind _output_get_3 (set `local.AppliedRotation` (* _output_get_2 (`KismetMathLibrary.SelectFloat` 1.0 -1.0 `TurnRight?`))))
  (`self.K2_AddActorLocalRotation` (`KismetMathLibrary.MakeRotator` 0.0 0.0 _output_get_3))
  (bind _output_get_4 (set `self.RotationRemaining` (- (`self.RotationRemaining`) (`local.DeltaRotation`))))
  (if (< _output_get_4 1.0)
    (set `self.RotationRemaining` 60.0)
    (set `self.IsRotating?` false)))

(fn `ToggleHandCollisions`
  (params (`TurnOff?` :type Boolean) (`Left?` :type Boolean))
  (if `TurnOff?`
    (if `Left?`
      (`PrimitiveComponent.SetCollisionEnabled` (`self.ArmHitBox_L`) "NoCollision")
      (else
        (`PrimitiveComponent.SetCollisionEnabled` (`self.ArmHitBox_R`) "NoCollision")))
    (elif `Left?`
      (`PrimitiveComponent.SetCollisionEnabled` (`self.ArmHitBox_L`) "QueryAndPhysics")
      (else
        (`PrimitiveComponent.SetCollisionEnabled` (`self.ArmHitBox_R`) "QueryAndPhysics")))))

(fn `UserConstructionScript`
  (bind _mesh (`self.Mesh`))
  (bind _returnvalue (* 1.0 (`self.MainBodyDamageMultiplier`)))
  (bind _returnvalue_2 (* 1.0 (`self.TentacleDamageMultiplier`)))
  (bind _returnvalue_3 (* 1.0 (`self.ArmsDamageMultiplier`)))
  (`parent.UserConstructionScript`)
  (`|ExecutionSequence`
    (:`then_0`
      (`SceneComponent.K2_AttachToComponent` (`self.ArmHitBox_R`) (`self.Mesh`) "Wrist_R" "KeepRelative" "KeepRelative" "KeepRelative" true)
      (`SceneComponent.K2_AttachToComponent` (`self.ArmHitBox_L`) (`self.Mesh`) "Wrist_L" "KeepRelative" "KeepRelative" "KeepRelative" true)
      (`SceneComponent.K2_AttachToComponent` (`self.MainBodyHitBox_neck`) (`self.Mesh`) "Neck2_M" "KeepRelative" "KeepRelative" "KeepRelative" true)
      (`SceneComponent.K2_AttachToComponent` (`self.TentSingleBACK_HitBox_1`) (`self.Mesh`) "BackTail0_M" "KeepRelative" "KeepRelative" "KeepRelative" true)
      (`SceneComponent.K2_AttachToComponent` (`self.TentSingleBACK_HitBox_2`) _mesh "BackTail2_M" "KeepRelative" "KeepRelative" "KeepRelative" true)
      (`SceneComponent.K2_AttachToComponent` (`self.TentSingleBACK_HitBox_3`) _mesh "BackTail3_M" "KeepRelative" "KeepRelative" "KeepRelative" true))
    (:`then_1`
      (`self.AttachCollidersToTentacles` (`self.TentFrontHitBox_R1`) "TentacleFront0_R" (`self.TentFrontHitBox_R2`) "TentacleFront2_R" (`self.TentFrontHitBox_R3`) "TentacleFront4_R" (`self.TentFrontHitBox_R4`) "TentacleFront5_R")
      (`self.AttachCollidersToTentacles` (`self.TentMiddleHitBox_R1`) "TentacleMiddle0_R" (`self.TentMiddleHitBox_R2`) "TentacleMiddle2_R" (`self.TentMiddleHitBox_R3`) "TentacleMiddle4_R" (`self.TentMiddleHitBox_R4`) "TentacleMiddle5_R")
      (`self.AttachCollidersToTentacles` (`self.TentBackHitBox_R1`) "TentacleBack0_R" (`self.TentBackHitBox_R2`) "TentacleBack2_R" (`self.TentBackHitBox_R3`) "TentacleBack4_R" (`self.TentBackHitBox_R4`) "TentacleBack5_R"))
    (:`then_2`
      (`self.AttachCollidersToTentacles` (`self.TentFrontHitBox_L1`) "TentacleFront0_L" (`self.TentFrontHitBox_L2`) "TentacleFront2_L" (`self.TentFrontHitBox_L3`) "TentacleFront4_L" (`self.TentFrontHitBox_L4`) "TentacleFront5_L")
      (`self.AttachCollidersToTentacles` (`self.TentMiddleHitBox_L1`) "TentacleMiddle0_L" (`self.TentMiddleHitBox_L2`) "TentacleMiddle2_L" (`self.TentMiddleHitBox_L3`) "TentacleMiddle4_L" (`self.TentMiddleHitBox_L4`) "TentacleMiddle5_L")
      (`self.AttachCollidersToTentacles` (`self.TentBackHitBox_L1`) "TentacleBack0_L" (`self.TentBackHitBox_L2`) "TentacleBack2_L" (`self.TentBackHitBox_L3`) "TentacleBack4_L" (`self.TentBackHitBox_L4`) "TentacleBack5_L"))
    (:`then_3`
      (set `self.HitBoxDamageMultipliers` (`|MakeMap` (`self.MainBodyHitBox`) _returnvalue (`self.ArmHitBox_R`) _returnvalue_3 (`self.ArmHitBox_L`) _returnvalue_3 (`self.TentFrontHitBox_R1`) _returnvalue_2 (`self.TentFrontHitBox_R2`) _returnvalue_2 (`self.TentFrontHitBox_R3`) _returnvalue_2 (`self.TentFrontHitBox_R4`) _returnvalue_2 (`self.TentMiddleHitBox_R1`) _returnvalue_2 (`self.TentMiddleHitBox_R2`) _returnvalue_2 (`self.TentMiddleHitBox_R3`) _returnvalue_2 (`self.TentMiddleHitBox_R4`) _returnvalue_2 (`self.TentBackHitBox_R1`) _returnvalue_2 (`self.TentBackHitBox_R2`) _returnvalue_2 (`self.TentBackHitBox_R3`) _returnvalue_2 (`self.TentBackHitBox_R4`) _returnvalue_2 (`self.TentFrontHitBox_L1`) _returnvalue_2 (`self.TentFrontHitBox_L2`) _returnvalue_2 (`self.TentFrontHitBox_L3`) _returnvalue_2 (`self.TentFrontHitBox_L4`) _returnvalue_2 (`self.TentMiddleHitBox_L1`) _returnvalue_2 (`self.TentMiddleHitBox_L2`) _returnvalue_2 (`self.TentMiddleHitBox_L3`) _returnvalue_2 (`self.TentMiddleHitBox_L4`) _returnvalue_2 (`self.TentBackHitBox_L1`) _returnvalue_2 (`self.TentBackHitBox_L2`) _returnvalue_2 (`self.TentBackHitBox_L3`) _returnvalue_2 (`self.TentBackHitBox_L4`) _returnvalue_2 (`self.TentSingleBACK_HitBox_1`) _returnvalue_2 (`self.TentSingleBACK_HitBox_2`) _returnvalue_2 (`self.TentSingleBACK_HitBox_3`) _returnvalue_2 :!type "PrimitiveComponent Object Reference"))
      (set `self.FinalDamgeMultiplier_Body` _returnvalue)
      (set `self.FinalDamgeMultiplier_Arms` _returnvalue_3)
      (set `self.FinalDamgeMultiplier_Tentacles` _returnvalue_2))))