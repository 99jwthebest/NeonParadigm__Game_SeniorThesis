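; Euphony boss enemy Blueprint that adds a boss health bar to the player's HUD on BeginPlay and refreshes it shortly after taking damage.
; Ground slam sphere-traces for pawns, then knocks the player away with an upward impulse, applies radial damage and temporarily ignores root motion until a timer resets it.
; Projectile attack fires from six arrow components toward randomly offset points around the player.
; Basic attack is a stub that only traces and casts.
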(event `self.ReceiveBeginPlay`
  (`KismetSystemLibrary.Delay` 0.02)
  (bind _returnvalue (`|CreateWidget` "/Game/_MyFiles/UI/WBP_BossHealthBar.WBP_BossHealthBar_C"))
  (bind _output_get (set `self.BossHealthBarWidget` _returnvalue))
  (set `/Game/_MyFiles/UI/WBP_BossHealthBar.EnemyBossOwner` self _output_get)
  (`/Game/_MyFiles/UI/WBP_BossHealthBar.UpdateHealth` _output_get)
  (bind _asbp_player_neon_paradigm (cast `/Game/_MyFiles/Blueprints/BP_Player_NeonParadigm` (`GameplayStatics.GetPlayerCharacter` 0)))
  (`VerticalBox.AddChildToVerticalBox` (`/Game/_MyFiles/UI/WBP_HUD.BossVerticalBox` (`/Game/_MyFiles/Blueprints/BP_Player_NeonParadigm.HudWidget` _asbp_player_neon_paradigm)) (`self.BossHealthBarWidget`)))

(event `self.ReceiveAnyDamage`
  (params (Damage :type "Float (single-precision)") (DamageType :type "DamageType Object Reference") (InstigatedBy :type "Controller Object Reference") (DamageCauser :type "Actor Object Reference"))
  (`KismetSystemLibrary.Delay` 0.02)
  (`/Game/_MyFiles/UI/WBP_BossHealthBar.UpdateHealth` (`self.BossHealthBarWidget`)))

(fn `PerformBasicAttack`
  (bind _returnvalue (`self.K2_GetActorLocation`))
  (bind (_outhit _returnvalue_2) (`KismetSystemLibrary.SphereTraceSingleForObjects` :`Start` _returnvalue :`End` _returnvalue :`Radius` 2000.0 :`ObjectTypes` (`|MakeArray` "ObjectTypeQuery3" :!type "EObjectTypeQuery Enum") :`DrawDebugType` "ForDuration"))
  (if _returnvalue_2
    (bind _asbp_player_neon_paradigm (cast `/Game/_MyFiles/Blueprints/BP_Player_NeonParadigm` (`GameplayStatics.GetPlayerCharacter` 0)))))

(fn `PerformGroundSlamAttack`
  (locals (KnockbackDirection :type "Vector Structure") (KnockbackImpulse :type "Vector Structure"))
  (bind _returnvalue (`self.K2_GetActorLocation`))
  (bind (_outhit _returnvalue_2) (`KismetSystemLibrary.SphereTraceSingleForObjects` :`Start` _returnvalue :`End` _returnvalue :`Radius` 2000.0 :`ObjectTypes` (`|MakeArray` "ObjectTypeQuery3" :!type "EObjectTypeQuery Enum") :`DrawDebugType` "ForDuration"))
  (if _returnvalue_2
    (bind _asbp_player_neon_paradigm (cast `/Game/_MyFiles/Blueprints/BP_Player_NeonParadigm` (`GameplayStatics.GetPlayerCharacter` 0)))
    (bind _output_get (set `local.KnockbackDirection` (`KismetMathLibrary.Normal` (- (`self.K2_GetActorLocation` _asbp_player_neon_paradigm) (`self.K2_GetActorLocation`)))))
    (bind _output_get_2 (set `local.KnockbackImpulse` (* (`KismetMathLibrary.MakeVector` (.x _output_get) (.y _output_get) 0.7) (`self.KnockbackForce`))))
    (`KismetSystemLibrary.PrintString` (`KismetStringLibrary.Conv_VectorToString` _output_get_2))
    (`CharacterMovementComponent.AddImpulse` (`Character.CharacterMovement` _asbp_player_neon_paradigm) _output_get_2 true)
    (`AnimInstance.SetRootMotionMode` (`SkeletalMeshComponent.GetAnimInstance` (`Character.Mesh` _asbp_player_neon_paradigm)) "IgnoreRootMotion")
    (`GameplayStatics.ApplyRadialDamage` :`BaseDamage` 100.0 :`Origin` _returnvalue :`DamageRadius` 2000.0 :`DamageTypeClass` "/Game/_MyFiles/Blueprints/NP_DamageTypes/NP_DT_Middle.NP_DT_Middle_C" :`DamageCauser` self :`InstigatedByController` (`self.GetInstigatorController`) :`bDoFullDamage` true)
    (`KismetSystemLibrary.K2_SetTimer` null "ReenablePlayerInput" 2.0)))

(fn `PerformShootProjectiles`
  (locals (RandomOffset :type "Vector Structure") (RandomTargetLocation :type "Vector Structure") (SpawnLocation :type "Vector Structure") (SpawnRotation :type "Rotator Structure"))
  (for _array_element (`|MakeArray` (`self.Arrow1`) (`self.Arrow2`) (`self.Arrow3`) (`self.Arrow4`) (`self.Arrow5`) (`self.Arrow6`))
    (if (not (not (`KismetSystemLibrary.IsValid` _array_element)))
      (set `local.RandomOffset` (* (`KismetMathLibrary.RandomUnitVector`) (`KismetMathLibrary.RandomFloatInRange` 0.0 (`self.TargetRadiusProjectiles`))))
      (bind _output_get (set `local.RandomTargetLocation` (+ (`self.K2_GetActorLocation` (`GameplayStatics.GetPlayerCharacter` 0)) (`local.RandomOffset`))))
      (bind _output_get_2 (set `local.SpawnLocation` (`SceneComponent.K2_GetComponentLocation` _array_element)))
      (bind _output_get_3 (set `local.SpawnRotation` (`KismetMathLibrary.FindLookAtRotation` _output_get_2 _output_get)))
      (`|SpawnActorFromClass` "/Game/_MyFiles/Blueprints/Projectiles/BP_Projectile.BP_Projectile_C" (`KismetMathLibrary.MakeTransform` _output_get_2 _output_get_3) "AdjustIfPossibleButAlwaysSpawn" "MultiplyWithRoot" self null)))
  (`KismetSystemLibrary.PrintString` "Yeah .!!!!!"))

(fn `ReenablePlayerInput`
  (bind _asbp_player_neon_paradigm (cast `/Game/_MyFiles/Blueprints/BP_Player_NeonParadigm` (`GameplayStatics.GetPlayerCharacter` 0)))
  (`AnimInstance.SetRootMotionMode` (`SkeletalMeshComponent.GetAnimInstance` (`Character.Mesh` _asbp_player_neon_paradigm)) "NoRootMotionExtraction")
  (`KismetSystemLibrary.PrintString` "Succeedded!!!!"))

(fn `UserConstructionScript`
  (`parent.UserConstructionScript`))