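; Ranged enemy Blueprint that fires magic shots at the player.
; FireProjectile spawns BP_MagicShot at the enemy's location, rotated toward the player character and owned by the enemy.
; It then casts the player to BP_Clair_NeonParadigm and stores itself in ProjectileCounterActorLoc, giving the player a reference to the shooter.
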(event `FireProjectile`
  (bind (_returnvalue_location _returnvalue_rotation _returnvalue_scale) (`KismetMathLibrary.BreakTransform` (`self.GetTransform`)))
  (bind _returnvalue (`GameplayStatics.GetPlayerCharacter` 0))
  (`|SpawnActorFromClass` "/Game/_MyFiles/Blueprints/Projectiles/BP_MagicShot.BP_MagicShot_C" (`KismetMathLibrary.MakeTransform` _returnvalue_location (`KismetMathLibrary.FindLookAtRotation` (`self.K2_GetActorLocation`) (`self.K2_GetActorLocation` _returnvalue)) _returnvalue_scale) "AdjustIfPossibleButAlwaysSpawn" "MultiplyWithRoot" self null)
  (bind _asbp_clair_neon_paradigm (cast `/Game/_MyFiles/Blueprints/BP_Clair_NeonParadigm` _returnvalue))
  (set `/Game/_MyFiles/Blueprints/BP_Clair_NeonParadigm.ProjectileCounterActorLoc` self _asbp_clair_neon_paradigm))

(fn `UserConstructionScript`
  (`parent.UserConstructionScript`))