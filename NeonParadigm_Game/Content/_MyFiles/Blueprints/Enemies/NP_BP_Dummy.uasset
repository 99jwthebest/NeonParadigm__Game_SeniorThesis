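; Dummy enemy character with a health bar widget, rhythm-delayed montage attacks and death cleanup that stops AI and movement.
; BeginPlay links the health bar after a short delay, and damage refreshes it.
; PerformAttack checks state and grounding, applies outline overlays, derives a delay from the montage's notify time, then plays it.
; DrawWeaponCollision sphere-traces forward, damaging each living player once per trace; attack events toggle indicator overlays.
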(event `self.ReceiveBeginPlay`
  (`KismetSystemLibrary.Delay` 0.02)
  (bind _aswbp_health_bar (cast `/Game/_MyFiles/UI/WBP_HealthBar` (`WidgetComponent.GetWidget` (`self.HealthBarWidget`))))
  ;[0.7865 0.04247 0] Sometimes there is a livecoding issue
  (set `/Game/_MyFiles/UI/WBP_HealthBar.EnemyOwner` self _aswbp_health_bar)
  (`/Game/_MyFiles/UI/WBP_HealthBar.UpdateHealth` _aswbp_health_bar)
  (set `self.HealthBarVar` _aswbp_health_bar))

(event `self.ReceiveAnyDamage`
  (params (Damage :type "Float (single-precision)") (DamageType :type "DamageType Object Reference") (InstigatedBy :type "Controller Object Reference") (DamageCauser :type "Actor Object Reference"))
  (`KismetSystemLibrary.Delay` 0.01)
  (`/Game/_MyFiles/UI/WBP_HealthBar.UpdateHealth` (`self.HealthBarVar`)))

(event `self.PerformThingsAfterDeath`
  (bind _returnvalue (`AIBlueprintHelperLibrary.GetAIController` self))
  (`BrainComponent.StopLogic` (`AIController.BrainComponent` _returnvalue) "")
  (`MovementComponent.StopMovementImmediately` (`self.CharacterMovement`))
  (`AIController.K2_ClearFocus` _returnvalue))

(event `StartAttack`
  (`MeshComponent.SetOverlayMaterial` (`self.Mesh`) "/Game/_MyFiles/Materials/M_EnemyIndicators/MI_Overlay_EnemyAttackIndicator.MI_Overlay_EnemyAttackIndicator"))

(event `EndAttack`
  (`MeshComponent.SetOverlayMaterial` (`self.Mesh`) null)
  (`MeshComponent.SetOverlayMaterial` (`self.WeaponMesh`) null))

(fn `CanAttack`
  (returns (ReturnValue :type Boolean))
  (bind _charactermovement (`self.CharacterMovement`))
  (return (and (not (`self.IsCurrentStateEqualToAny` (`|MakeArray` "Attack" "Dodge" "Death" "Disabled" :!type "ECharacterStates Enum"))) (not (or (`NavMovementComponent.IsFalling` _charactermovement) (`NavMovementComponent.IsFlying` _charactermovement))))))

(fn `DrawWeaponCollision`
  (params (End :type "Float (single-precision)") (Radius :type "Float (single-precision)") (DamageTypeClass :type "NP_DamageType Class Reference") (AmountOfDamage :type "Float (double-precision)"))
  (bind _returnvalue (`self.K2_GetActorLocation`))
  (`KismetArrayLibrary.Array_Clear` (`self.HitActors`))
  ;[0.02083 0.02083 0.02083] Collision
  (bind (_outhits _returnvalue_2) (`KismetSystemLibrary.SphereTraceMultiForObjects` _returnvalue (+ (* (`self.GetActorForwardVector`) End) _returnvalue) Radius (`|MakeArray` "ObjectTypeQuery3" :!type "EObjectTypeQuery Enum")))
  (if _returnvalue_2
    ;[0.02083 0.02083 0.02083] Check Each Actor Hit
    (for _array_element _outhits
      (bind (_bblockinghit _binitialoverlap _time _distance _location _impactpoint _normal _impactnormal _physmat _hitactor) (`GameplayStatics.BreakHitResult` _array_element))
      ;[0.02083 0.02083 0.02083] Hit Actor Cannot Be In The Array and Has To Be Valid To Take Damage
      (if (and (not (`KismetArrayLibrary.Array_Contains` (`self.HitActors`) _hitactor)) (`KismetSystemLibrary.IsValid` _hitactor))
        (bind _asbp_player_neon_paradigm (cast `/Game/_MyFiles/Blueprints/BP_Player_NeonParadigm` _hitactor))
        (if (`|EnumInequality` (`CharacterStateComponent.GetState` (`NeonParadigm_GameCharacter.CharacterState` _asbp_player_neon_paradigm)) "Death")
          (`GameplayStatics.ApplyDamage` _hitactor (`local.AmountOfDamage`) (`self.GetController`) self (`local.DamageTypeClass`))
          (`KismetArrayLibrary.Array_AddUnique` (`self.HitActors`) _hitactor))))))

(fn `PerformAttack`
  (params (Index :type Integer))
  (returns (ReturnValue :type "Float (single-precision)"))
  (bind _output (`|GetArrayItem` (`self.Attack Montages`) Index))
  (if (`self.CanAttack`)
    (`/Engine/EditorBlueprintResources/StandardMacros.IsValid` _output
      (:`Is Valid`
        (`MeshComponent.SetOverlayMaterial` (`self.WeaponMesh`) "/Game/_MyFiles/Materials/M_EnemyIndicators/M_OutlineBIG_Yellow_Enemy.M_OutlineBIG_Yellow_Enemy")
        (`MeshComponent.SetOverlayMaterial` (`self.Mesh`) "/Game/_MyFiles/Materials/M_EnemyIndicators/M_OutlineBIG_Yellow_Enemy.M_OutlineBIG_Yellow_Enemy")
        ;[1 0 0] Might Need to change the notify for Ranged attackers to work
        (`self.FindNotifyTriggerTime` _output (select `bool` (`self.bCanBeParried`) :`false` (`self.RangedNotifyName`) :`true` (`self.MeleeNotifyName`)))
        (`self.SetCurrentAnimTimeDelay` (`self.GetNotifyTriggerTime`))
        (`self.TestRhythmDelayEvent`)
        (`self.SetState` "Attack")
        (bind _returnvalue (`AnimInstance.Montage_Play` (`SkeletalMeshComponent.GetAnimInstance` (`self.Mesh`)) _output (`self.GetCurrentAnimPlayRate`) "Duration" 0.0 true))
        (return _returnvalue))
      (:`Is Not Valid`
        (return 0.0)))
    (else
      (return 0.0))))

(fn `UserConstructionScript`)