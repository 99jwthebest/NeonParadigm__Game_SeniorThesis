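; BP_Clair_NeonParadigm is an actor Blueprint that owns the health HUD and refreshes it when the actor takes damage.
; On BeginPlay, it waits briefly, creates a WBP_HUD widget, adds it to the viewport and updates the health display.
; AnyDamage calls the same health update after a short delay, with no health math in this graph.
; An unconnected self-damage node never runs.
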(event `self.ReceiveBeginPlay`
  (`KismetSystemLibrary.Delay` 0.01)
  (bind _returnvalue (`|CreateWidget` "/Game/_MyFiles/UI/WBP_HUD.WBP_HUD_C"))
  (bind _output_get (set `self.HudWidget` _returnvalue))
  (`UserWidget.AddToViewport` _output_get 0)
  (`/Game/_MyFiles/UI/WBP_HUD.UpdateHealth` _output_get))

(event `Key|F`
  (params (Key :type "Key Structure")))

(event `self.ReceiveAnyDamage`
  (params (Damage :type "Float (single-precision)") (DamageType :type "DamageType Object Reference") (InstigatedBy :type "Controller Object Reference") (DamageCauser :type "Actor Object Reference"))
  (`KismetSystemLibrary.Delay` 0.01)
  (`/Game/_MyFiles/UI/WBP_HUD.UpdateHealth` (`self.HUDWidget`)))

(fn `UserConstructionScript`)