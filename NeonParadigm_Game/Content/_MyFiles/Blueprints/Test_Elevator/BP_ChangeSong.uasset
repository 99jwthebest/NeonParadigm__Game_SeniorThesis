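; BP_ChangeSong is a trigger actor in the elevator test folder that signals the FMOD music actor when the player enters its box.
; Box overlap accepts only BP_Player_NeonParadigm, stores the player reference and calls ChangeSong.
; ChangeSong finds the first BP_NP_FMOD_Music in the level, sets its FirstTimeBool to false and prints a debug string.
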(event `self.Box.OnComponentBeginOverlap`
  (params (OverlappedComponent :type "PrimitiveComponent Object Reference") (OtherActor :type "Actor Object Reference") (OtherComp :type "PrimitiveComponent Object Reference") (OtherBodyIndex :type Integer) (bFromSweep :type Boolean) (SweepResult :type "HitResult Structure (by ref)"))
  (bind _asbp_player_neon_paradigm (cast `/Game/_MyFiles/Blueprints/BP_Player_NeonParadigm` OtherActor))
  (set `self.Player` _asbp_player_neon_paradigm)
  (`self.ChangeSong`))

(event `ChangeSong`
  (bind _outactors (`GameplayStatics.GetAllActorsOfClass` "/Game/_MyFiles/Blueprints/FMOD/BP_NP_FMOD_Music.BP_NP_FMOD_Music_C"))
  (bind _output_get (set `self.BP_FMOD_in` (`|GetArrayItem` _outactors)))
  (bind _asbp_np_fmod_music (cast `/Game/_MyFiles/Blueprints/FMOD/BP_NP_FMOD_Music` _output_get))
  (bind _output_get_2 (set `self.As BP NP FMOD Music` _asbp_np_fmod_music))
  (`NP_FMOD_Music.SetFirstTimeBool` _output_get_2 false)
  (`KismetSystemLibrary.PrintString` "HEYYYYYYYYY"))

(fn `UserConstructionScript`)