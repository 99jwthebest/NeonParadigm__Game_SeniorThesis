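; BP_SoundBars is an actor that builds a row of instanced cubes with a material driven by music tempo.
; On BeginPlay, after a short delay, it spaces instances along local Y and creates a dynamic M_CubesMoving material.
; SetBPM passes a tempo to that material's BPM parameter.
; It also caches the level's BP_NP_FMOD_Music actor, though this graph never uses it.
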(event `self.ReceiveBeginPlay`
  (`KismetSystemLibrary.Delay` 0.02)
  (for _index (range 1 (`self.CubesInstancesCount`))
    (bind _output_get (set `self.InstanceLocation` (`KismetMathLibrary.MakeVector` 0.0 (* _index 10.0))))
    (bind _output_get_2 (set `self.InstanceTransform` (`KismetMathLibrary.MakeTransform` _output_get)))
    (`InstancedStaticMeshComponent.AddInstance` (`self.InstancedStaticMesh`) _output_get_2 false))
  (bind _returnvalue (`PrimitiveComponent.CreateDynamicMaterialInstance` (`self.InstancedStaticMesh`) 0 "/Game/_MyFiles/Materials/M_CubesMoving.M_CubesMoving" "None"))
  (set `self.YeahDMI` _returnvalue)
  (bind _outactors (`GameplayStatics.GetAllActorsOfClass` "/Game/_MyFiles/Blueprints/FMOD/BP_NP_FMOD_Music.BP_NP_FMOD_Music_C"))
  (bind _output_get_3 (set `self.BP_FMOD_in` (`|GetArrayItem` _outactors)))
  (bind _asbp_np_fmod_music (cast `/Game/_MyFiles/Blueprints/FMOD/BP_NP_FMOD_Music` _output_get_3))
  (set `self.As BP NP FMOD Music` _asbp_np_fmod_music))

(fn `SetBPM`
  (params (`New BPM` :type "Float (double-precision)"))
  (bind _yeahdmi (`self.YeahDMI`)
    (:`then`
      (`MaterialInstanceDynamic.SetScalarParameterValue` _yeahdmi "BPM" `New BPM`))
    (:`else`)))

(fn `UserConstructionScript`)