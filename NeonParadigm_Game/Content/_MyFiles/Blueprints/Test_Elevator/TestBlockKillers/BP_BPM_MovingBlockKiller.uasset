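; BP_BPM_MovingBlockKiller is a hazard block, in an elevator test folder, that hurts the player and sends them back to a spawn point.
; Overlapping ActualPlayerHurtCollision with BP_Player_NeonParadigm applies damage, prints a debug string and moves the player to the SpawnPoint actor's location.
; Level sequence playback for looping the MovingBlockAnim at a raised play rate is present but disconnected, so this graph does not move the block.
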(event `self.ReceiveBeginPlay`)

(event `self.StaticMesh.OnComponentHit`
  (params (HitComponent :type "PrimitiveComponent Object Reference") (OtherActor :type "Actor Object Reference") (OtherComp :type "PrimitiveComponent Object Reference") (NormalImpulse :type "Vector Structure") (Hit :type "HitResult Structure (by ref)")))

(event `self.StaticMesh.OnComponentBeginOverlap`
  (params (OverlappedComponent :type "PrimitiveComponent Object Reference") (OtherActor :type "Actor Object Reference") (OtherComp :type "PrimitiveComponent Object Reference") (OtherBodyIndex :type Integer) (bFromSweep :type Boolean) (SweepResult :type "HitResult Structure (by ref)")))

(event `self.ActualPlayerHurtCollision.OnComponentBeginOverlap`
  (params (OverlappedComponent :type "PrimitiveComponent Object Reference") (OtherActor :type "Actor Object Reference") (OtherComp :type "PrimitiveComponent Object Reference") (OtherBodyIndex :type Integer) (bFromSweep :type Boolean) (SweepResult :type "HitResult Structure (by ref)"))
  (bind _asbp_player_neon_paradigm (cast `/Game/_MyFiles/Blueprints/BP_Player_NeonParadigm` OtherActor))
  (`GameplayStatics.ApplyDamage` _asbp_player_neon_paradigm 100.0)
  (`KismetSystemLibrary.PrintString` "Hello" true true (struct :`R` 1.0 :`B` 0.500774 :`A` 1.0))
  (`self.K2_SetActorLocation` _asbp_player_neon_paradigm (`self.K2_GetActorLocation` (`self.SpawnPoint`)) false false))

(fn `UserConstructionScript`)