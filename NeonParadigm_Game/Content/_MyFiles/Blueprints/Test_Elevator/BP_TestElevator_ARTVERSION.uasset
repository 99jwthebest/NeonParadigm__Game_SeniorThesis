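; Test elevator actor that, on player interaction, alternates between rising a fixed height and returning to its start position.
; Interact advances a floor counter to pick the target, then Tick moves the actor there with constant-speed VInterpTo until within a small tolerance.
; Four barriers turn visible and solid during travel, then hide on arrival.
; Debug prints remain, and the three floor positions computed at BeginPlay are never used for movement.
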(event `self.ReceiveBeginPlay`
  (bind _arrayofbarrieractors (`self.ArrayOfBarrierActors`))
  (bind _output_get (set `self.StartVec` (`self.K2_GetActorLocation`)))
  (bind _output_get_2 (set `self.ElevatorFloor1` _output_get))
  (bind _output_get_3 (set `self.ElevatorFloor2` (+ _output_get_2 (0.0 0.0 3500.0))))
  (set `self.ElevatorFloor3` (+ _output_get_3 (0.0 0.0 2000.0)))
  (`KismetArrayLibrary.Array_Add` (`self.ArrayOfBarrierActors`) (`self.Barrier`))
  (`KismetArrayLibrary.Array_Add` _arrayofbarrieractors (`self.Barrier1`))
  (`KismetArrayLibrary.Array_Add` _arrayofbarrieractors (`self.Barrier2`))
  (`KismetArrayLibrary.Array_Add` _arrayofbarrieractors (`self.Barrier3`))
  (for _array_element _arrayofbarrieractors
    (`PrimitiveComponent.SetCollisionEnabled` _array_element "NoCollision")
    (`SceneComponent.SetHiddenInGame` _array_element true false)))

(event `self.Box.OnComponentBeginOverlap`
  (params (OverlappedComponent :type "PrimitiveComponent Object Reference") (OtherActor :type "Actor Object Reference") (OtherComp :type "PrimitiveComponent Object Reference") (OtherBodyIndex :type Integer) (bFromSweep :type Boolean) (SweepResult :type "HitResult Structure (by ref)")))

(event `self.Interact`
  (bind _asbp_player_neon_paradigm (cast `/Game/_MyFiles/Blueprints/BP_Player_NeonParadigm` (`GameplayStatics.GetPlayerCharacter` 0)))
  (set `self.Player` _asbp_player_neon_paradigm)
  (`KismetSystemLibrary.PrintString` "Yay!!!" true true (struct :`R` 1.0 :`B` 0.172135 :`A` 1.0))
  (bind _result (`/Engine/EditorBlueprintResources/StandardMacros.IncrementInt` (`self.FloorCount`))
    (:`  `
      (bind _output_get (set `self.FloorCount` _result))
      (`KismetSystemLibrary.PrintString` (`KismetStringLibrary.Conv_IntToString` _output_get) true true (struct :`R` 1.0 :`B` 0.172135 :`A` 1.0))
      (if (>= (`self.FloorCount`) 2)
        (bind _output_get_2 (set `self.FloorCount` 0))
        (`KismetSystemLibrary.PrintString` (`KismetStringLibrary.Conv_IntToString` _output_get_2) true true (struct :`R` 1.0 :`B` 0.172135 :`A` 1.0))
        (set `self.TargetVec` (`self.StartVec`))
        (`self.ElevatorMoveFunc`)
        (else
          (`self.SetElevatorVectors`)
          (`self.ElevatorMoveFunc`))))))

(event `self.ReceiveTick`
  (params (DeltaSeconds :type "Float (single-precision)"))
  (if (`self.bElevatorMoving`)
    (`self.ElevatorMoveFunc`)))

(event `ElevatorMoveFunc`
  (bind _returnvalue (`KismetMathLibrary.Vector_Distance` (`self.K2_GetActorLocation`) (`self.TargetVec`)))
  (set `self.bElevatorMoving` true)
  (for _array_element (`self.ArrayOfBarrierActors`)
    (`PrimitiveComponent.SetCollisionEnabled` _array_element "QueryAndPhysics")
    (`SceneComponent.SetHiddenInGame` _array_element false false))
  (if (<= (`self.FloorCount`) 0)
    (bind _returnvalue_2 (`KismetMathLibrary.VInterpTo_Constant` (`self.K2_GetActorLocation`) (`self.TargetVec`) (stale `self.ReceiveTick` DeltaSeconds) 750.0))
    (`self.K2_SetActorLocation` _returnvalue_2)
    (if (<= _returnvalue 50.0)
      (set `self.bElevatorMoving` false)
      (`KismetSystemLibrary.PrintString` (`KismetStringLibrary.Conv_DoubleToString` _returnvalue))
      (for _array_element_2 (`self.ArrayOfBarrierActors`) :!label _label
        (`PrimitiveComponent.SetCollisionEnabled` _array_element_2 "NoCollision")
        (`SceneComponent.SetHiddenInGame` _array_element_2 true false)))
    (else
      (`self.K2_SetActorLocation` _returnvalue_2)
      (if (<= (`KismetMathLibrary.Vector_Distance` (`self.K2_GetActorLocation`) (`self.TargetVec`)) 50.0)
        (set `self.bElevatorMoving` false)
        (goto _label)))))

(event `SetElevatorVectors`
  (if (<= (`self.FloorCount`) 1)
    (bind _output_get (set `self.ElevatorMoveVector` (0.0 0.0 3500.0)))
    (set `self.TargetVec` (+ _output_get (`self.K2_GetActorLocation`)))
    (`KismetSystemLibrary.PrintString` "not supPOSED  to be here!!!" true true (struct :`R` 0.944918 :`G` 1.0 :`A` 1.0))
    (else
      (`KismetSystemLibrary.PrintString` "supposed to be here!!!")
      (bind _output_get_2 (set `self.ElevatorMoveVector` (0.0 0.0 3500.0)))
      (set `self.TargetVec` (+ _output_get_2 (`self.K2_GetActorLocation`))))))

(fn `UserConstructionScript`)