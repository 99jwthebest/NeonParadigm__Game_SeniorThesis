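; Trigger actor, apparently in a test elevator area, that reactivates a set of wall actors when the player enters its box.
; The box overlap casts to BP_Player_NeonParadigm, stores the player and calls ActivateLight, which despite its name unhides each CurrentWallActors entry and enables its collision, once only via DoOnce.
; A disconnected debug branch that would stop the player's area sequences based on combat encounter count never runs.
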(event `self.Box.OnComponentBeginOverlap`
  (params (OverlappedComponent :type "PrimitiveComponent Object Reference") (OtherActor :type "Actor Object Reference") (OtherComp :type "PrimitiveComponent Object Reference") (OtherBodyIndex :type Integer) (bFromSweep :type Boolean) (SweepResult :type "HitResult Structure (by ref)"))
  (bind _asbp_player_neon_paradigm (cast `/Game/_MyFiles/Blueprints/BP_Player_NeonParadigm` OtherActor))
  (set `self.Player` _asbp_player_neon_paradigm)
  (`self.ActivateLight`))

(event `ActivateLight`
  (`/Engine/EditorBlueprintResources/StandardMacros.DoOnce` false
    (:`Completed`
      (for _array_element (`self.CurrentWallActors`)
        (`self.SetActorHiddenInGame` _array_element false)
        (`self.SetActorEnableCollision` _array_element true)))))

(fn `UserConstructionScript`)