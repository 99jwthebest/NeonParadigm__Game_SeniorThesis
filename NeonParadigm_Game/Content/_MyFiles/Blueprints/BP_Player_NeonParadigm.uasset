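; Player character Blueprint for Neon Paradigm, a music-synced combat game, handling HUD, menus, camera and interaction.
; Update events refresh HUD bars, score and grade, while FMOD tempo drives beat animations, a looping Level Sequence and sound bars.
; Tick smooths the detached camera boom, varying vertical speed by fall state and elevator overlap.
; An overlap sphere enables interaction; debug keys, prints and disconnected parry-spawn and weapon-trace logic remain.
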(event `Key|Four`
  (params (Key :type "Key Structure"))
  (:`Pressed`
    (`/Game/_MyFiles/UI/WBP_HUD.ToggleBPMBarHelper` (`self.HudWidget`))))

(event `Key|T`
  (params (Key :type "Key Structure"))
  (:`Pressed`
    (`GameplayStatics.OpenLevelBySoftObjectPtr` "/Game/_MyFiles/Levels/LevelDesign.LevelDesign")))

(event `Key|Escape` :paused true
  (params (Key :type "Key Structure"))
  ;[1 0.1975 0] We might be able to put all this in c++
)

(event `Key|P` :paused true
  (params (Key :type "Key Structure"))
  (bind _returnvalue (`GameplayStatics.GetPlayerController` 0))
  (bind _returnvalue_2 (`GameplayStatics.GetPlayerController` 0))
  ;[1 0.1975 0] We might be able to put all this in c++
  (:`Pressed`
    (if (not (`self.isPauseMenuOpened`))
      (set `self.isPauseMenuOpened` true)
      (bind _returnvalue_3 (`|CreateWidget` "/Game/_MyFiles/UI/MenuUI/WBP_PauseMenu.WBP_PauseMenu_C" _returnvalue_2))
      (bind _output_get (set `self.PauseMenuWidget` _returnvalue_3))
      (`UserWidget.AddToViewport` _output_get 0)
      (`WidgetBlueprintLibrary.SetInputMode_GameAndUIEx` _returnvalue_2 (`self.PauseMenuWidget`))
      (set `PlayerController.bShowMouseCursor` true (`GameplayStatics.GetPlayerController` 0))
      (`GameplayStatics.SetGamePaused` true)
      (else
        (set `self.isPauseMenuOpened` false)
        (`Widget.RemoveFromParent` (`self.PauseMenuWidget`))
        (`GameplayStatics.SetGamePaused` false)
        (`WidgetBlueprintLibrary.SetInputMode_GameOnly` _returnvalue)
        (set `PlayerController.bShowMouseCursor` false _returnvalue)))))

(event `Key|One`
  (params (Key :type "Key Structure")))

(event `self.ReceiveBeginPlay`
  (bind _hudwidget (`self.HudWidget`))
  (`SceneComponent.K2_SetWorldLocation` (`self.CameraBoom`) (`self.K2_GetActorLocation`) false false)
  (`KismetSystemLibrary.Delay` 0.01)
  (bind _returnvalue (`|CreateWidget` "/Game/_MyFiles/UI/WBP_HUD.WBP_HUD_C"))
  (bind _output_get (set `self.HudWidget` _returnvalue))
  (`UserWidget.AddToViewport` _output_get 0)
  (`/Game/_MyFiles/UI/WBP_HUD.UpdateHealth` _output_get)
  (`/Game/_MyFiles/UI/WBP_HUD.UpdateRageBar` _hudwidget)
  (`/Game/_MyFiles/UI/WBP_HUD.UpdateScore` _hudwidget)
  (`/Game/_MyFiles/UI/WBP_HUD.UpdateGradeLetter` _hudwidget)
  (`/Game/_MyFiles/UI/WBP_HUD.ToggleStyleGradeBox` _hudwidget)
  (`/Game/_MyFiles/UI/WBP_HUD.TogglePerfectHitTextBox` _hudwidget)
  (`/Game/_MyFiles/UI/WBP_HUD.UpdateRankLetterProgress` _hudwidget)
  (`/Game/_MyFiles/UI/WBP_HUD.UpdateProjectileWeaponBar` _hudwidget)
  (`/Game/_MyFiles/UI/WBP_HUD.UpdateProjectileWeaponStunBar` _hudwidget)
  (`/Game/_MyFiles/UI/WBP_HUD.UpdateDodgeCooldown` _hudwidget))

(event `self.OnLanded`
  (params (Hit :type "HitResult Structure (by ref)"))
  (if Hit_bBlockingHit
    (bind _output_get (set `self.CurrentCamZMoveValue` 2.0))
    (`KismetSystemLibrary.PrintString` (`KismetStringLibrary.Conv_DoubleToString` _output_get))))

(event `self.UpdateBPM_Visuals`
  (`MovieSceneSequencePlayer.Stop` (stale `self.BeginBPM_Bar` _output_get))
  (bind _output (`|GetArrayItem` (stale `self.BeginBPM_Bar` _outactors)))
  (bind _returnvalue (`NP_FMOD_Music.GetGlobalTempo` (`/Game/_MyFiles/Blueprints/Test_Elevator/BP_SoundBars.As BP NP FMOD Music` _output)))
  (bind _returnvalue_2 (/ _returnvalue 60.0))
  (`KismetSystemLibrary.PrintString` (`KismetStringLibrary.Conv_DoubleToString` _returnvalue_2) true true (struct :`G` 0.66 :`B` 1.0 :`A` 1.0) 10.0)
  (`KismetSystemLibrary.PrintString` (`KismetStringLibrary.Conv_DoubleToString` _returnvalue) true true (struct :`G` 0.66 :`B` 1.0 :`A` 1.0) 10.0)
  (`MovieSceneSequencePlayer.SetPlayRate` (stale `self.BeginBPM_Bar` _output_get) _returnvalue_2)
  (`MovieSceneSequencePlayer.PlayLooping` (stale `self.BeginBPM_Bar` _output_get) -1)
  (`/Game/_MyFiles/UI/WBP_HUD.PlayBPMHalfCircleAnim` (`self.HudWidget`) _returnvalue_2 :!label _label)
  (`/Game/_MyFiles/Blueprints/Test_Elevator/BP_SoundBars.SetBPM` _output _returnvalue)
  (`/Game/_MyFiles/Blueprints/Test_Elevator/BP_SoundBars.SetHeight` _output 200.0))

(event `self.PlayBPM_BallAnim`
  (bind _returnvalue (/ (`self.GetCurrentTempoDelay`) 2.0))
  (`KismetSystemLibrary.PrintString` (`KismetStringLibrary.Conv_DoubleToString` _returnvalue) true true (struct :`R` 1.0 :`B` 0.014722 :`A` 1.0))
  (`KismetSystemLibrary.K2_SetTimerDelegate` (delegate `PlayBPMHalfCircleBlueprint`) _returnvalue))

(event `self.ReceiveAnyDamage`
  (params (Damage :type "Float (single-precision)") (DamageType :type "DamageType Object Reference") (InstigatedBy :type "Controller Object Reference") (DamageCauser :type "Actor Object Reference"))
  (`KismetSystemLibrary.Delay` 0.01)
  (`/Game/_MyFiles/UI/WBP_HUD.UpdateHealth` (`self.HUDWidget`)))

(event `self.BeginBPM_Bar`
  (bind _outactors (`GameplayStatics.GetAllActorsOfClass` "/Game/_MyFiles/Blueprints/Test_Elevator/BP_SoundBars.BP_SoundBars_C"))
  (bind _returnvalue (/ (`NP_FMOD_Music.GetGlobalTempo` (`/Game/_MyFiles/Blueprints/Test_Elevator/BP_SoundBars.As BP NP FMOD Music` (`|GetArrayItem` _outactors))) 60.0))
  (bind (_outactor _returnvalue_2) (`LevelSequencePlayer.CreateLevelSequencePlayer` "/Game/_MyFiles/Blueprints/Test_Elevator/TestAnims/MovingBlockAnim.MovingBlockAnim" (make `MovieSceneSequencePlaybackSettings` false (struct) _returnvalue)))
  (bind _output_get (set `self.NewVar` _returnvalue_2))
  (`MovieSceneSequencePlayer.PlayLooping` _output_get -1)
  (`MovieSceneSequencePlayer.SetPlayRate` _output_get _returnvalue)
  (goto _label))

(event `PlayBPMHalfCircleBlueprint`
  (bind _returnvalue (`self.GetCurrentUIBallAnimPlayRate`))
  (`/Game/_MyFiles/UI/WBP_HUD.PlayBPMBallAnim` (`self.HudWidget`) _returnvalue)
  (`KismetSystemLibrary.PrintString` (`KismetStringLibrary.Conv_DoubleToString` _returnvalue) true true (struct :`R` 1.0 :`B` 0.014722 :`A` 1.0)))

(event `self.ReceiveTick`
  (params (DeltaSeconds :type "Float (single-precision)"))
  (bind _returnvalue (`GameplayStatics.GetWorldDeltaSeconds`))
  (bind _returnvalue_2 (`self.K2_GetActorLocation`))
  (bind (_returnvalue_x _returnvalue_y _returnvalue_z) (`KismetMathLibrary.BreakVector` (`self.GetVelocity`)))
  (bind (_returnvalue_x_2 _returnvalue_y_2 _returnvalue_z_2) (`KismetMathLibrary.BreakVector` (`self.GetVelocity`)))
  (bind _currentcamzmovevalue (`self.CurrentCamZMoveValue`))
  (bind _cameraboom (`self.CameraBoom`))
  (bind (_returnvalue_x_3 _returnvalue_y_3 _returnvalue_z_3) (`KismetMathLibrary.BreakVector` (`SceneComponent.K2_GetComponentLocation` _cameraboom)))
  (bind (_returnvalue_x_4 _returnvalue_y_4) (`KismetMathLibrary.BreakVector` (`KismetMathLibrary.VInterpTo` (`KismetMathLibrary.MakeVector` _returnvalue_x_3 _returnvalue_y_3) _returnvalue_2 _returnvalue 20.0)))
  (bind _output_get (set `self.CurrentCamZMoveValue` (select `bool` (> _returnvalue_z -400.0) :`false` (`KismetMathLibrary.FInterpTo` _currentcamzmovevalue 10.0 _returnvalue 8.0) :`true` (select `bool` (and (> _returnvalue_z_2 -400.0) (not (`NavMovementComponent.IsFalling` (`self.CharacterMovement`)))) :`false` (`KismetMathLibrary.FInterpTo` _currentcamzmovevalue 2.0 _returnvalue 6.0) :`true` (`KismetMathLibrary.FInterpTo` _currentcamzmovevalue 6.0 _returnvalue 6.0) :!type "Float (single-precision)") :!type "Float (single-precision)")))
  (bind (_returnvalue_x_5 _returnvalue_y_5 _returnvalue_z_4) (`KismetMathLibrary.BreakVector` (`KismetMathLibrary.VInterpTo` (`KismetMathLibrary.MakeVector` 0.0 0.0 _returnvalue_z_3) _returnvalue_2 _returnvalue (`KismetMathLibrary.SelectFloat` 30.0 _output_get (`self.bOnElevator`)))))
  (`SceneComponent.K2_SetWorldLocation` _cameraboom (`KismetMathLibrary.MakeVector` _returnvalue_x_4 _returnvalue_y_4 _returnvalue_z_4) false false))

(event `self.ParryProjectile`
  (cast `/Game/_MyFiles/Blueprints/NP_DamageTypes/NP_DT_Projectile` (stale `self.ReceiveAnyDamage` DamageType)
    (:`then`
      (`self.Counter` true)
      (`KismetSystemLibrary.PrintString` "We DID ITT!!!!")
      (set `self.ProjectileCounterActorLoc` null))
    (:`CastFailed`
      (`KismetSystemLibrary.PrintString` "yuhhh!!!!"))))

(event `SpawnWinMenu`
  (bind _returnvalue (`|CreateWidget` "/Game/_MyFiles/UI/MenuUI/WBP_WinMenu.WBP_WinMenu_C" (`GameplayStatics.GetPlayerController` 0)))
  (`UserWidget.AddToViewport` _returnvalue 0))

(event `self.SetBPM_SoundBarsHeight`
  (bind _output (`|GetArrayItem` (stale `self.BeginBPM_Bar` _outactors)))
  (`/Game/_MyFiles/Blueprints/Test_Elevator/BP_SoundBars.SetHeight` _output (select `bool` (== (`/Game/_MyFiles/Blueprints/Test_Elevator/BP_SoundBars.CurrentHeight` _output) 200.0) :`false` 200.0 :`true` 100.0)))

(event `self.SpawnLoseMenu`
  (bind _returnvalue (`|CreateWidget` "/Game/_MyFiles/UI/MenuUI/WBP_LoseMenu.WBP_LoseMenu_C" (`GameplayStatics.GetPlayerController` 0)))
  (`UserWidget.AddToViewport` _returnvalue 0))

(event `self.UpdateRageBarEvent`
  (`/Game/_MyFiles/UI/WBP_HUD.UpdateRageBar` (`self.HudWidget`)))

(event `self.UpdateHealthBarEvent`
  (`/Game/_MyFiles/UI/WBP_HUD.UpdateHealth` (`self.HudWidget`)))

(event `self.UpdateScoreEvent`
  (bind _hudwidget (`self.HudWidget`))
  (`/Game/_MyFiles/UI/WBP_HUD.UpdateScore` _hudwidget)
  (`/Game/_MyFiles/UI/WBP_HUD.UpdateGradeLetter` _hudwidget)
  (`/Game/_MyFiles/UI/WBP_HUD.UpdateRankLetterProgress` _hudwidget))

(event `self.ToggleCombatStyleGrade`
  (`/Game/_MyFiles/UI/WBP_HUD.ToggleStyleGradeBox` (`self.HudWidget`)))

(event `self.PlayBPM_HalfCirle`
  (params (CurrentTempo :type "Float (single-precision)"))
  (`/Game/_MyFiles/UI/WBP_HUD.PlayBPMHalfCircleAnim` (`self.HudWidget`) (/ (/ CurrentTempo 60.0) 2.0)))

(event `self.TogglePerfectHitTextBox`
  (`/Game/_MyFiles/UI/WBP_HUD.TogglePerfectHitTextBox` (`self.HudWidget`)))

(event `self.ToggleEncounterResults`
  (`/Game/_MyFiles/UI/WBP_HUD.ToggleFinalResultsCombatEncounter` (`self.HudWidget`)))

(event `self.UpdateProjectileWeaponBarEvent`
  (`/Game/_MyFiles/UI/WBP_HUD.UpdateProjectileWeaponBar` (`self.HudWidget`)))

(event `self.UpdateProjectileWeaponStunBarEvent`
  (`/Game/_MyFiles/UI/WBP_HUD.UpdateProjectileWeaponStunBar` (`self.HudWidget`)))

(event `self.UpdateDodgeBarEvent`
  (`/Game/_MyFiles/UI/WBP_HUD.UpdateDodgeCooldown` (`self.HudWidget`)))

(event `self.UpdateMaxHealthBarEvent`
  (`/Game/_MyFiles/UI/WBP_HUD.UpdateMaxHealthBar` (`self.HudWidget`)))

(event `Key|Two`
  (params (Key :type "Key Structure"))
  (:`Pressed`
    (`GameplayStatics.PlaySoundAtLocation` "/Game/_MyFiles/SoundFX/SoundFX_NeonParadigm_TestHitSoundDelay4th.SoundFX_NeonParadigm_TestHitSoundDelay4th" (`self.K2_GetActorLocation`) (struct) 2.5 1.1 0.05 null null null null)))

(event `self.UpdateMaxRageBarEvent`
  (`/Game/_MyFiles/UI/WBP_HUD.UpdateMaxRageBar` (`self.HudWidget`)))

(event `self.SpawnWinMenuEvent`
  (`self.SpawnWinMenu`))

(event `self.InteractableSphereCollision.OnComponentBeginOverlap`
  (params (OverlappedComponent :type "PrimitiveComponent Object Reference") (OtherActor :type "Actor Object Reference") (OtherComp :type "PrimitiveComponent Object Reference") (OtherBodyIndex :type Integer) (bFromSweep :type Boolean) (SweepResult :type "HitResult Structure (by ref)"))
  (bind _asbp_interact (cast `/Game/_MyFiles/Blueprints/Test_Elevator/BP_Interact` OtherActor))
  (set `self.As BP Interact` _asbp_interact)
  (`KismetSystemLibrary.PrintString` "ElevatorCanActivate!!!!" true true (struct :`R` 1.0 :`G` 0.86627 :`A` 1.0))
  (set `self.bOnElevator` true))

(event `self.InteractableSphereCollision.OnComponentEndOverlap`
  (params (OverlappedComponent :type "PrimitiveComponent Object Reference") (OtherActor :type "Actor Object Reference") (OtherComp :type "PrimitiveComponent Object Reference") (OtherBodyIndex :type Integer))
  (set `self.As BP Interact` null)
  (`KismetSystemLibrary.PrintString` "ElevatorCanNOTActivate!!!!" true true (struct :`R` 1.0 :`G` 0.227507 :`A` 1.0))
  (set `self.bOnElevator` false))

(event `Key|Y`
  (params (Key :type "Key Structure"))
  (bind _as_bp_interact (`self.As BP Interact`))
  (:`Pressed`
    (`/Engine/EditorBlueprintResources/StandardMacros.IsValid` (`KismetSystemLibrary.Conv_InterfaceToObject` _as_bp_interact)
      (:`Is Valid`
        (`/Game/_MyFiles/Blueprints/Test_Elevator/BP_Interact.Interact` _as_bp_interact)))))

(fn `TestProjectileWeaponCollision`
  (`self.PlayAnimMontage` "/Game/_MyFiles/Animation/Assets/Attacks/Ranged/AM_ProjectileWeapon.AM_ProjectileWeapon"))

(fn `UserConstructionScript`)