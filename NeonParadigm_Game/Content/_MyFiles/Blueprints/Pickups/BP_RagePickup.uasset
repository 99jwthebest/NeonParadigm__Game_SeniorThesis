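; Rage pickup that grants the player a fixed amount of rage and destroys itself when collected.
; Hitting a static mesh actor switches off mesh physics, while hitting the player collects it directly.
; Once physics is off, Tick interpolates it toward the player while their magnetize dodge is active, collecting it within a set distance.
; Leftover disconnected experiments and a debug print remain.
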(event `self.ReceiveTick`
  (params (DeltaSeconds :type "Float (single-precision)"))
  (bind _asbp_player_neon_paradigm (cast `/Game/_MyFiles/Blueprints/BP_Player_NeonParadigm` (`GameplayStatics.GetPlayerCharacter` 0)))
  (if (and (`NeonParadigm_GameCharacter.bIsMagnetizeDodgeActive` _asbp_player_neon_paradigm) (not (`SceneComponent.IsSimulatingPhysics` (`self.StaticMesh`) "None")))
    (bind _returnvalue (`self.K2_GetActorLocation` _asbp_player_neon_paradigm))
    (`self.K2_SetActorLocation` (`KismetMathLibrary.VInterpTo` (`self.K2_GetActorLocation`) _returnvalue DeltaSeconds (`self.MagnetizationSpeed`)))
    (if (< (`KismetMathLibrary.Vector_Distance` (`self.K2_GetActorLocation`) _returnvalue) (`self.Ball Dissappear Distance`))
      (`NeonParadigm_GameCharacter.AddToCurrentRage` _asbp_player_neon_paradigm 20.0)
      (`self.K2_DestroyActor`))))

(event `self.StaticMesh.OnComponentBeginOverlap`
  (params (OverlappedComponent :type "PrimitiveComponent Object Reference") (OtherActor :type "Actor Object Reference") (OtherComp :type "PrimitiveComponent Object Reference") (OtherBodyIndex :type Integer) (bFromSweep :type Boolean) (SweepResult :type "HitResult Structure (by ref)")))

(event `self.StaticMesh.OnComponentHit`
  (params (HitComponent :type "PrimitiveComponent Object Reference") (OtherActor :type "Actor Object Reference") (OtherComp :type "PrimitiveComponent Object Reference") (NormalImpulse :type "Vector Structure") (Hit :type "HitResult Structure (by ref)"))
  (if (== (`GameplayStatics.GetObjectClass` OtherActor) "/Script/Engine.StaticMeshActor")
    (`PrimitiveComponent.SetSimulatePhysics` (`self.StaticMesh`) false)
    (`KismetSystemLibrary.PrintString` (`KismetStringLibrary.Conv_BoolToString` (`SceneComponent.IsSimulatingPhysics` (`self.StaticMesh`) "None")))
    (else
      (bind _asbp_player_neon_paradigm (cast `/Game/_MyFiles/Blueprints/BP_Player_NeonParadigm` OtherActor))
      (`NeonParadigm_GameCharacter.AddToCurrentRage` _asbp_player_neon_paradigm 20.0)
      (`self.K2_DestroyActor`))))

(fn `UserConstructionScript`)