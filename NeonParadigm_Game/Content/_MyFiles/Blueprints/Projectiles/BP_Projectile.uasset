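; BP_Projectile is a projectile that damages the Neon Paradigm player when its box overlaps them.
; It skips players in i-frames or the Death state; otherwise it applies NP_DT_Projectile damage, spawns an explosion and destroys itself.
; Static mesh actors also trigger the explosion, spawned at that actor's origin rather than the contact point.
; A timed self-destruct exists but is unconnected, so a projectile that hits nothing is not destroyed here.
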(event `self.ReceiveBeginPlay`)

(event `self.Box.OnComponentBeginOverlap`
  (params (OverlappedComponent :type "PrimitiveComponent Object Reference") (OtherActor :type "Actor Object Reference") (OtherComp :type "PrimitiveComponent Object Reference") (OtherBodyIndex :type Integer) (bFromSweep :type Boolean) (SweepResult :type "HitResult Structure (by ref)"))
  (bind _asbp_player_neon_paradigm (cast `/Game/_MyFiles/Blueprints/BP_Player_NeonParadigm` OtherActor)
    (:`then`
      (if (and (not (`NeonParadigm_GameCharacter.IsIFramesEnabled` _asbp_player_neon_paradigm)) (`|EnumInequality` (`CharacterStateComponent.GetState` (`NeonParadigm_GameCharacter.CharacterState` _asbp_player_neon_paradigm)) "Death"))
        (`GameplayStatics.ApplyDamage` _asbp_player_neon_paradigm (`self.Base Damage`) null null "/Game/_MyFiles/Blueprints/NP_DamageTypes/NP_DT_Projectile.NP_DT_Projectile_C")
        (`/Engine/EditorBlueprintResources/StandardMacros.IsValid` _asbp_player_neon_paradigm
          (:`Is Valid`
            (`GameplayStatics.SpawnEmitterAtLocation` "/Game/StarterContent/Particles/P_Explosion.P_Explosion" (`self.K2_GetActorLocation` _asbp_player_neon_paradigm))
            (`self.K2_DestroyActor`)))))
    (:`CastFailed`
      (if (== (`GameplayStatics.GetObjectClass` OtherActor) "/Script/Engine.StaticMeshActor")
        (`GameplayStatics.SpawnEmitterAtLocation` "/Game/StarterContent/Particles/P_Explosion.P_Explosion" (`self.K2_GetActorLocation` OtherActor))
        (`self.K2_DestroyActor`)))))

(fn `UserConstructionScript`)