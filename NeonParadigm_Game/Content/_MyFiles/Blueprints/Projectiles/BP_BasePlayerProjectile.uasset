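; Base player projectile that damages dummy enemies (NP_BP_Dummy) on contact and explodes.
; Its Box overlap casts to the dummy, ignores it in the Death state, and otherwise applies BaseDamage with the projectile's owner as damage causer.
; A successful hit spawns an explosion emitter at the dummy's location and destroys the projectile.
; Other actors are ignored, as the static mesh impact branch is disconnected and never runs.
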(event `self.Box.OnComponentBeginOverlap`
  (params (OverlappedComponent :type "PrimitiveComponent Object Reference") (OtherActor :type "Actor Object Reference") (OtherComp :type "PrimitiveComponent Object Reference") (OtherBodyIndex :type Integer) (bFromSweep :type Boolean) (SweepResult :type "HitResult Structure (by ref)"))
  (bind _asnp_bp_dummy (cast `/Game/_MyFiles/Blueprints/Enemies/NP_BP_Dummy` OtherActor))
  (if (`|EnumInequality` (`NP_BaseEnemy.CurrentState` _asnp_bp_dummy) "Death")
    (`GameplayStatics.ApplyDamage` _asnp_bp_dummy (`self.Base Damage`) null (`self.GetOwner`))
    (`GameplayStatics.SpawnEmitterAtLocation` "/Game/StarterContent/Particles/P_Explosion.P_Explosion" (`self.K2_GetActorLocation` _asnp_bp_dummy))
    (`self.K2_DestroyActor`)))

(fn `UserConstructionScript`)