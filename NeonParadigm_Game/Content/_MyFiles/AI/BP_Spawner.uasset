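; BP_Spawner is a trigger actor that spawns a configured set of enemies, once, when the player enters its box.
; Each class in the EnemiesToSpawn map spawns its mapped count at random navigable points within Radius, yawed toward the player.
; Every spawned enemy registers with the level's BP_NP_FMOD_Music actor.
; Each player overlap also toggles the HUD style grade box, outside the one-time guard.
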(event `self.ReceiveBeginPlay`
  (bind _asbp_neon_game_instance (cast `/Game/_MyFiles/Blueprints/GameInstance/BP_NeonGameInstance` (`GameplayStatics.GetGameInstance`)))
  (set `self.As BP Neon Game Instance` _asbp_neon_game_instance))

(event `self.Box.OnComponentBeginOverlap`
  (params (OverlappedComponent :type "PrimitiveComponent Object Reference") (OtherActor :type "Actor Object Reference") (OtherComp :type "PrimitiveComponent Object Reference") (OtherBodyIndex :type Integer) (bFromSweep :type Boolean) (SweepResult :type "HitResult Structure (by ref)"))
  (bind _asbp_player_neon_paradigm (cast `/Game/_MyFiles/Blueprints/BP_Player_NeonParadigm` OtherActor))
  (bind _output_get (set `self.Player` _asbp_player_neon_paradigm))
  (`self.Spawn`)
  (`/Game/_MyFiles/UI/WBP_HUD.ToggleStyleGradeBox` (`/Game/_MyFiles/Blueprints/BP_Player_NeonParadigm.HudWidget` _output_get)))

(event `Spawn`
  (bind _enemiestospawn (`self.EnemiesToSpawn`))
  (`/Engine/EditorBlueprintResources/StandardMacros.DoOnce` false
    (:`Completed`
      (`self.GetFModMusic`)
      (bind _keys (`BlueprintMapLibrary.Map_Keys` _enemiestospawn))
      (for _array_element _keys
        (for _ (range 1 (+ (`BlueprintMapLibrary.Map_Find` _enemiestospawn _array_element) 1))
          (`KismetSystemLibrary.PrintString` "EnemySpawning")
          (bind _randomlocation (`NavigationSystemV1.K2_GetRandomLocationInNavigableRadius` (`self.K2_GetActorLocation`) (`self.Radius`) null null))
          (bind _returnvalue (`|SpawnActorFromClass` _array_element (`KismetMathLibrary.MakeTransform` _randomlocation) "AdjustIfPossibleButAlwaysSpawn" "MultiplyWithRoot" null null))
          (bind (_returnvalue_roll _returnvalue_pitch) (`KismetMathLibrary.BreakRotator` (`self.K2_GetActorRotation` _returnvalue)))
          (bind (_returnvalue_roll_2 _returnvalue_pitch_2 _returnvalue_yaw) (`KismetMathLibrary.BreakRotator` (`KismetMathLibrary.FindLookAtRotation` (`self.K2_GetActorLocation` _returnvalue) (`self.K2_GetActorLocation` (`self.Player`)))))
          (`self.K2_SetActorRotation` _returnvalue (`KismetMathLibrary.MakeRotator` _returnvalue_roll _returnvalue_pitch _returnvalue_yaw) false)
          (`NP_FMOD_Music.AddSpawnedEnemy` (`self.As BP NP FMOD Music`) _returnvalue))))))

(fn `GetFModMusic`
  (bind _outactors (`GameplayStatics.GetAllActorsOfClass` "/Game/_MyFiles/Blueprints/FMOD/BP_NP_FMOD_Music.BP_NP_FMOD_Music_C"))
  (bind _output_get (set `self.BP_FMOD_in` (`|GetArrayItem` _outactors)))
  (bind _asbp_np_fmod_music (cast `/Game/_MyFiles/Blueprints/FMOD/BP_NP_FMOD_Music` _output_get))
  (set `self.As BP NP FMOD Music` _asbp_np_fmod_music))

(fn `UserConstructionScript`)