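; Boss AI controller that drives an NP_BP_Dummy pawn through that pawn's own behavior tree and periodically triggers attacks.
; On possess it runs the tree, then seeds the blackboard with player character 0 as target and a strafe distance.
; A looping timer, whose random interval is rolled only once at possession, calls PerformAttack to switch the blackboard behavior state and set the save-attack flag.
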(event `PerformAttack`
  (bind _returnvalue (`AIBlueprintHelperLibrary.GetBlackboard` self))
  (`/Engine/EditorBlueprintResources/StandardMacros.IsValid` _returnvalue
    (:`Is Valid`
      (`BlackboardComponent.SetValueAsEnum` _returnvalue (`self.StateKeyName`) (cast `/Game/_MyFiles/Blueprints/Enums/E_BehaviorStates` (enumliteral `/Game/_MyFiles/Blueprints/Enums/E_BehaviorStates` "NewEnumerator3")))
      (`BlackboardComponent.SetValueAsBool` _returnvalue (`self.SaveAttackKeyName`) true))))

(event `self.ReceivePossess`
  (params (PossessedPawn :type "Pawn Object Reference"))
  (bind _asnp_bp_dummy (cast `/Game/_MyFiles/Blueprints/Enemies/NP_BP_Dummy` PossessedPawn))
  (`self.RunBehaviorTree` self (`/Game/_MyFiles/Blueprints/Enemies/NP_BP_Dummy.BT_BehaviorTree` _asnp_bp_dummy))
  (`self.SetBlackboardKeys`)
  (`KismetSystemLibrary.K2_SetTimerDelegate` (delegate `PerformAttack`) (`KismetMathLibrary.RandomFloatInRange` 3.0 (`self.MaxAttackWaitTime`)) true))

(fn `SetBlackboardKeys`
  (bind _returnvalue (`AIBlueprintHelperLibrary.GetBlackboard` self))
  (`/Engine/EditorBlueprintResources/StandardMacros.IsValid` _returnvalue
    (:`Is Valid`
      (`BlackboardComponent.SetValueAsObject` _returnvalue (`self.TargetKeyName`) (`GameplayStatics.GetPlayerCharacter` 0))
      (`BlackboardComponent.SetValueAsFloat` _returnvalue (`self.StrafeDistanceKeyName`) (`self.StrafeDistance`)))))

(fn `UserConstructionScript`)