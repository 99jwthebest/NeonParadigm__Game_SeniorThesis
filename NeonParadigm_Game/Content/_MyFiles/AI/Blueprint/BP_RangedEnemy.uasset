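; BP_RangedEnemy is a ranged enemy that shoots magic projectiles at the player.
; Its FireProjectile event spawns BP_MagicShot at the enemy's location, rotated toward player 0's current position, with the enemy as owner; nothing in this graph calls it.
; A disconnected fragment that would register the enemy as BP_NeonParadigm_Clair's ProjectileCounterActorLoc never runs.
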(event `FireProjectile`
  (bind (_returnvalue_location _returnvalue_rotation _returnvalue_scale) (`KismetMathLibrary.BreakTransform` (`self.GetTransform`)))
  (`|SpawnActorFromClass` "/Game/_MyFiles/Blueprints/Projectiles/BP_MagicShot.BP_MagicShot_C" (`KismetMathLibrary.MakeTransform` _returnvalue_location (`KismetMathLibrary.FindLookAtRotation` (`self.K2_GetActorLocation`) (`self.K2_GetActorLocation` (`GameplayStatics.GetPlayerCharacter` 0))) _returnvalue_scale) "AdjustIfPossibleButAlwaysSpawn" "MultiplyWithRoot" self null))

(fn `UserConstructionScript`
  (`parent.UserConstructionScript`))