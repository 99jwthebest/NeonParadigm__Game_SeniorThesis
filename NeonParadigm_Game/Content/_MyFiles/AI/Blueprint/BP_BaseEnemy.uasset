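; BP_BaseEnemy is a base enemy character with health, lock-on indicators, a simple state machine and montage-driven attacks.
; Damage triggers death or a directional hit-reaction montage chosen by damage type, turning it toward the attacker with timeline-driven backward knockback.
; Attacks are gated by state and grounding, while a forward sphere trace damages the Clair player character.
; The HealthBar assignment is disconnected, and StartAttack and EndAttack are empty stubs.
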(event `OnTargeted`
  (`SceneComponent.SetVisibility` (`self.Widget`) true false)
  (`SceneComponent.SetVisibility` (`self.TargetLockOn`) true false))

(event `self.ReceiveBeginPlay`
  (set `self.CurrentHealth` (`self.MaxHealth`))
  (bind _aswbp_health_bar (cast `/Game/_MyFiles/UI/WBP_HealthBar` (`WidgetComponent.GetWidget` (`self.Widget`)))))

(event `EndTarget`
  (`SceneComponent.SetVisibility` (`self.Widget`) false false)
  (`SceneComponent.SetVisibility` (`self.TargetLockOn`) false false))

(event `self.ReceiveAnyDamage`
  (params (Damage :type "Float (single-precision)") (DamageType :type "DamageType Object Reference") (InstigatedBy :type "Controller Object Reference") (DamageCauser :type "Actor Object Reference"))
  (bind (_returnvalue_roll _returnvalue_pitch) (`KismetMathLibrary.BreakRotator` (`self.K2_GetActorRotation`)))
  (bind (_returnvalue_roll_2 _returnvalue_pitch_2 _returnvalue_yaw) (`KismetMathLibrary.BreakRotator` (`KismetMathLibrary.FindLookAtRotation` (`self.K2_GetActorLocation`) (`self.K2_GetActorLocation` DamageCauser))))
  ;[0.02083 0.02083 0.02083] Take Damage
  (bind _output_get (set `self.CurrentHealth` (- (`self.CurrentHealth`) Damage)))
  (`/Game/_MyFiles/UI/WBP_HealthBar.UpdateHealth` (`self.HealthBar`))
  (if (> _output_get 0.0)
    (bind _asbp_damage_type_main (cast `/Game/_MyFiles/Blueprints/DamageType/BP_DamageTypeMain` DamageType))
    (bind _newparam (`self.GetHitReaction` (`/Game/_MyFiles/Blueprints/DamageType/BP_DamageTypeMain.DamageType` _asbp_damage_type_main)))
    ;[1 0 0] Need to add Hit Reaction Animations for this branch to work
    (if (and (not (`self.IsCurrentStateEqualToAny` (`|MakeArray` "NewEnumerator3" :!type "/Game/_MyFiles/Blueprints/Enums/E_State Enum"))) (`KismetSystemLibrary.IsValid` _newparam))
      (`self.SetState` "NewEnumerator4")
      (`self.K2_SetActorRotation` (`KismetMathLibrary.MakeRotator` _returnvalue_roll _returnvalue_pitch _returnvalue_yaw))
      (`self.StopAttackMovement`)
      ;[0.02083 0.02083 0.02083] 25 in distance parameter.
      (`self.AttackMovement` 500.0)
      (`self.PlayAnimMontage` _newparam)
      (else
        (`KismetSystemLibrary.PrintString` "ENEMY HIT REACTION IS NOT VALID" true true (struct :`R` 1.0 :`B` 0.1104 :`A` 1.0))))
    (else
      (`self.PerformDeath`))))

(event `AttackMovement`
  (params (Distance :type "Float (single-precision)"))
  (bind _returnvalue (`self.K2_GetActorLocation`))
  ;[0.008184 0.1562 0] Attack Movement
  (`self.StopAttackMovement`)
  (if (!= Distance 0.0)
    (bind (_direction _alpha) (`Timeline|Timeline` :!via `PlayFromStart` :!label _label)
      (:`Update`
        ;;[1 1 1] Update Character's Location
        (`self.K2_SetActorLocation` (`KismetMathLibrary.VLerp` _returnvalue (+ _returnvalue (* (* (`self.GetActorForwardVector`) -1.0) Distance)) _alpha) true)))))

(event `StopAttackMovement`
  ;[0.008184 0.1562 0] Attack Movement
  (goto _label :!via `Stop`))

(event `ResetState`
  (`self.SetState` "NewEnumerator0"))

(event `StartAttack`
  ;[1 0 0] Create Material Overlay with video, part 21, 47 minutes
)

(event `EndAttack`
  ;[1 0 0] Create Material Overlay with video, part 21, 47 minutes
)

(fn `CanAttack`
  (returns (ReturnValue :type Boolean))
  (bind _charactermovement (`self.CharacterMovement`))
  (return (and (not (`self.IsCurrentStateEqualToAny` (`|MakeArray` "NewEnumerator1" "NewEnumerator2" "NewEnumerator3" "NewEnumerator4" :!type "/Game/_MyFiles/Blueprints/Enums/E_State Enum"))) (not (or (`NavMovementComponent.IsFalling` _charactermovement) (`NavMovementComponent.IsFlying` _charactermovement))))))

(fn `DrawWeaponCollision`
  (params (End :type "Float (single-precision)") (Radiius :type "Float (single-precision)") (DamageTypeClass :type "/Game/_MyFiles/Blueprints/DamageType/BP_DamageTypeMain Class Reference") (AmountOfDamage :type "Float (double-precision)"))
  (bind _returnvalue (`self.K2_GetActorLocation`))
  (`KismetArrayLibrary.Array_Clear` (`self.HitActors`))
  ;[0.02083 0.02083 0.02083] Collision
  (bind (_outhits _returnvalue_2) (`KismetSystemLibrary.SphereTraceMultiForObjects` :`Start` _returnvalue :`End` (+ (* (`self.GetActorForwardVector`) End) _returnvalue) :`Radius` Radiius :`ObjectTypes` (`|MakeArray` "ObjectTypeQuery3" :!type "EObjectTypeQuery Enum") :`DrawDebugType` "ForDuration"))
  (if _returnvalue_2
    ;[0.02083 0.02083 0.02083] Check Each Actor Hit
    (for _array_element _outhits
      (bind (_bblockinghit _binitialoverlap _time _distance _location _impactpoint _normal _impactnormal _physmat _hitactor) (`GameplayStatics.BreakHitResult` _array_element))
      ;[0.02083 0.02083 0.02083] Hit Actor Cannot Be In The Array and Has To Be Valid To Take Damage
      (if (and (not (`KismetArrayLibrary.Array_Contains` (`self.HitActors`) _hitactor)) (`KismetSystemLibrary.IsValid` _hitactor))
        (bind _asbp_neon_paradigm_clair (cast `/Game/_MyFiles/Blueprints/Test_Elevator/BP_NeonParadigm_Clair` _hitactor))
        (if (`|EnumInequality` (`/Game/_MyFiles/Blueprints/Test_Elevator/BP_NeonParadigm_Clair.GetState` _asbp_neon_paradigm_clair) "NewEnumerator3")
          (`GameplayStatics.ApplyDamage` _hitactor (`local.AmountOfDamage`) (`self.GetController`) self (`local.DamageTypeClass`))
          (`KismetArrayLibrary.Array_AddUnique` (`self.HitActors`) _hitactor))))))

(fn `GetHitReaction`
  (params (DamageType :type "/Game/_MyFiles/Blueprints/Enums/E_DamageTypes Enum" :default "NewEnumerator0"))
  (returns (NewParam :type "AnimMontage Object Reference"))
  (switch `/Game/_MyFiles/Blueprints/Enums/E_DamageTypes` DamageType
    (:`NewEnumerator0`
      (return null))
    (:`NewEnumerator1`
      (return (`self.HR_Right`)))
    (:`NewEnumerator2`
      (return (`self.HR_Left`)))
    (:`NewEnumerator3`
      (return (`self.HR_Middle`)))
    (:`NewEnumerator4`
      (return (`self.HR_Knockdown`)))
    (:`NewEnumerator5`
      (return (`self.HR_Knockback`)))))

(fn `GetState`
  (returns (ReturnValue :type "/Game/_MyFiles/Blueprints/Enums/E_State Enum"))
  (return (`self.CurrentState`)))

(fn `IsCurrentStateEqualToAny`
  (params (StatesToCheck :type "Array of /Game/_MyFiles/Blueprints/Enums/E_State Enum (by ref)"))
  (returns (ReturnValue :type Boolean))
  (return (`KismetArrayLibrary.Array_Contains` StatesToCheck (`self.CurrentState`))))

(fn `PerformAttack`
  (params (Index :type Integer))
  (returns (ReturnValue :type "Float (single-precision)"))
  (bind _output (`|GetArrayItem` (`self.AttackMontages`) Index))
  (if (`self.CanAttack`)
    (`/Engine/EditorBlueprintResources/StandardMacros.IsValid` _output
      (:`Is Valid`
        (`self.SetState` "NewEnumerator1")
        (bind _returnvalue (`AnimInstance.Montage_Play` (`SkeletalMeshComponent.GetAnimInstance` (`self.Mesh`)) _output 1.0 "Duration" 0.0 true))
        (return _returnvalue))
      (:`Is Not Valid`
        (return 0.0)))
    (else
      (return 0.0))))

(fn `PerformDeath`
  (`self.SetState` "NewEnumerator3")
  (`self.PlayAnimMontage` (`self.DeathMontage`))
  (`PrimitiveComponent.SetCollisionEnabled` (`self.CapsuleComponent`) "NoCollision")
  (`PrimitiveComponent.SetCollisionEnabled` (`self.Mesh`) "NoCollision"))

(fn `SetState`
  (params (NewState :type "/Game/_MyFiles/Blueprints/Enums/E_State Enum" :default "NewEnumerator0"))
  (if (`|EnumInequality` NewState (`self.CurrentState`))
    (set `self.CurrentState` NewState)))

(fn `UserConstructionScript`)