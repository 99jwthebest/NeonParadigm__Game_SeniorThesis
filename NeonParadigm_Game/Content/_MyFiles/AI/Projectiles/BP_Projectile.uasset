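; BP_Projectile is an AI projectile that damages the BP_NeonParadigm_Clair character on contact.
; Its Box overlap applies damage to that character unless invincibility frames are active or the character is in one specific excluded state.
; Overlapping a StaticMeshActor instead spawns an explosion particle at the sweep's impact point.
; The graph contains no movement or destroy logic.
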(event `self.Box.OnComponentBeginOverlap`
  (params (OverlappedComponent :type "PrimitiveComponent Object Reference") (OtherActor :type "Actor Object Reference") (OtherComp :type "PrimitiveComponent Object Reference") (OtherBodyIndex :type Integer) (bFromSweep :type Boolean) (SweepResult :type "HitResult Structure (by ref)"))
  (bind _asbp_neon_paradigm_clair (cast `/Game/_MyFiles/Blueprints/BP_NeonParadigm_Clair` OtherActor)
    (:`then`
      (if (and (not (`/Game/_MyFiles/Blueprints/BP_NeonParadigm_Clair.IsIFramesEnabled` _asbp_neon_paradigm_clair)) (`|EnumInequality` (`/Game/_MyFiles/Blueprints/BP_NeonParadigm_Clair.GetState` _asbp_neon_paradigm_clair) "NewEnumerator3"))
        (`GameplayStatics.ApplyDamage` _asbp_neon_paradigm_clair)))
    (:`CastFailed`
      (if (== (`GameplayStatics.GetObjectClass` OtherActor) "/Script/Engine.StaticMeshActor")
        (`GameplayStatics.SpawnEmitterAtLocation` "/Game/StarterContent/Particles/P_Explosion.P_Explosion" (`.ImpactPoint` (`GameplayStatics.BreakHitResult` SweepResult)))))))

(fn `UserConstructionScript`)